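; PMF team replication info actor that represents one team, tracking its player PRIs, win count and squads.
; On BeginPlay it spawns one squad replication info actor per squad name from the game logic, stored for lookup by index.
; Join and leave update the player list, with joining also stamping the team index on the PRI.
; Respawning is denied for the spectator team, and wins also increment the Pavlov team score when that mode is enabled.
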(event EventBeginPlay
  (|CallParentFunction)
  (Squads|GenerateSquads))

(fn ConstructionScript)

(fn PlayerJoinTeam
  (params (PRI :type PMF%20Player%20Replication%20Info%20Object%20Reference))
  (Utilities|Array|AddUnique (Variables|DataReplicated|GetTeamPRIs) PRI)
  (Variables|/Game/CustomMaps/UGC1908549791/PMF/Blueprints/Info/PMF_PlayerReplicationInfo.PMF_PlayerReplicationInfo_C|SetTeamIndex PRI (Variables|DataReplicated|GetTeamIndex)))

(fn PlayerLeaveTeam
  (params (PRI :type PMF%20Player%20Replication%20Info%20Object%20Reference))
  (Utilities|Array|RemoveItem (Variables|DataReplicated|GetTeamPRIs) PRI))

(fn GetPlayerCount
  (return (Utilities|Array|Length (Variables|DataReplicated|GetTeamPRIs))))

(fn CanPlayerRespawn
  (params (PRI :type PMF%20Player%20Replication%20Info%20Object%20Reference))
  (return (!= (Variables|DataReplicated|GetTeamIndex) (Variables|/Game/CustomMaps/UGC1908549791/PMF/Blueprints/Data/Objects/PMF_GlobalVariables.PMF_GlobalVariables_C|GetTeamSpectatorIndex (CallFunction|GetPMFGlobals)))))

(fn HasAnyPlayers
  (return (> (Info|GetPlayerCount) 0)))

(fn AddWins
  (bind _pmfgamelogic (CallFunction|GetPMFGameLogic))
  (Utilities|FlowControl|Sequence
    (:then_0
      (Math|Integer|IncrementInt (Variables|DataReplicated|GetTeamWins)))
    (:then_1
      (if (Variables|/Game/CustomMaps/UGC1908549791/PMF/Blueprints/LevelActors/CORE/PMF_GameLogic.PMF_GameLogic_C|GetUsePavlovTeams _pmfgamelogic)
        (Class|PavlovGameLogic|IncrementTeamScore _pmfgamelogic (Math|Conversions|ToInteger(Byte) (Variables|DataReplicated|GetTeamIndex)) 1)))))

(fn GenerateSquads
  (bind _pmfgamelogic (CallFunction|GetPMFGameLogic))
  (bind _squadreplicationinfoclass (Variables|/Game/CustomMaps/UGC1908549791/PMF/Blueprints/LevelActors/CORE/PMF_GameLogic.PMF_GameLogic_C|GetSquadReplicationInfoClass _pmfgamelogic))
  (if (!= _squadreplicationinfoclass 0)
    (for (_array_element _array_index) (Variables|/Game/CustomMaps/UGC1908549791/PMF/Blueprints/LevelActors/CORE/PMF_GameLogic.PMF_GameLogic_C|GetSquadNames _pmfgamelogic)
      (bind _returnvalue (Game|SpawnActorfromClass _squadreplicationinfoclass (Math|Transform|MakeTransform "0, 0, 0") "AlwaysSpawn" 0 (Math|Conversions|ToByte(Integer) _array_index) _array_element 0))
      (Utilities|Array|AddUnique (Variables|DataReplicated|GetAllSRIs) _returnvalue))))

(fn GetSquadbyIndex
  (params (SquadIndex :type Byte))
  (if (Utilities|Array|IsValidIndex (Variables|DataReplicated|GetAllSRIs) (Math|Conversions|ToInteger(Byte) SquadIndex))
    (return true (Utilities|Array|Get(acopy) (Variables|DataReplicated|GetAllSRIs) (Math|Conversions|ToInteger(Byte) SquadIndex)))
    (else
      (return false 0))))