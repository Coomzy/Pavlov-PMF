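; Per-player proxy actor for the PMF framework that applies player rules and movement modifiers to the owning character.
; Once a pawn exists, the server applies vitality, cash, buying and loadout settings, and binds empty damage hooks.
; OwningCharacter's OnRep initializes clients with overhead visuals, speed, overlaps and inputs.
; Opt-in server/local/remote ticks drive local airborne gravity and velocity limits, alongside jump, item-restriction and VR yaw-corrected teleport helpers.
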(event Custom|ClientSetLocAndRot
  (params (Loc :type Vector) (Yaw :type Float%20%28single-precision%29))
  (bind _owningpri (Variables|DataReplicated|GetOwningPRI))
  (bind _vrcamera (Default|GetVRHeadsetCamera _owningpri))
  (Utilities|IsValid _vrcamera
    (:Is%20Valid
      (Transformation|SetActorLocationAndRotation (Variables|DataReplicated|GetOwningCharacter) Loc (Math|Rotator|MakeRotator 0.0 0.0 (- Yaw (.Yaw (Math|Rotator|BreakRotator (Variables|/Script/Engine.SceneComponent|GetRelativeRotation _vrcamera))))) false true))
    (:Is%20Not%20Valid
      (CallFunction|ClientSetLocandRotPlaySpace Loc Yaw))))

(event Custom|RegisterCharacterDamageEvents
  (bind _owningcharacter (Variables|DataReplicated|GetOwningCharacter))
  ;[1 1 1] Character Binds
  (EventDispatchers|AssignOnTakeAnyDamage _owningcharacter (delegate Custom|Bind_OnTakeAnyDamage))
  (EventDispatchers|AssignOnTakePointDamage _owningcharacter (delegate Custom|Bind_OnTakePointDamage))
  (EventDispatchers|AssignOnTakeRadialDamage _owningcharacter (delegate Custom|Bind_OnTakeRadialDamage)))

(event Custom|Bind_OnTakeAnyDamage
  (params (DamagedActor :type Actor%20Object%20Reference) (Damage :type Float%20%28single-precision%29) (DamageType :type Damage%20Type%20Object%20Reference) (InstigatedBy :type Controller%20Object%20Reference) (DamageCauser :type Actor%20Object%20Reference))
  ;[1 1 1] Character Binds
  (CharacterBinds|CharacteronTakeAnyDamage DamagedActor Damage DamageType InstigatedBy DamageCauser))

(event Custom|Bind_OnTakePointDamage
  (params (DamagedActor :type Actor%20Object%20Reference) (Damage :type Float%20%28single-precision%29) (InstigatedBy :type Controller%20Object%20Reference) (HitLocation :type Vector) (FHitComponent :type Primitive%20Component%20Object%20Reference) (BoneName :type Name) (ShotFromDirection :type Vector) (DamageType :type Damage%20Type%20Object%20Reference) (DamageCauser :type Actor%20Object%20Reference))
  ;[1 1 1] Character Binds
  (CharacterBinds|CharacteronTakePointDamage DamagedActor Damage InstigatedBy HitLocation FHitComponent BoneName ShotFromDirection DamageType DamageCauser))

(event Custom|Bind_OnTakeRadialDamage
  (params (DamagedActor :type Actor%20Object%20Reference) (Damage :type Float%20%28single-precision%29) (DamageType :type Damage%20Type%20Object%20Reference) (Origin :type Vector) (HitInfo :type Hit%20Result%20Structure) (InstigatedBy :type Controller%20Object%20Reference) (DamageCauser :type Actor%20Object%20Reference))
  ;[1 1 1] Character Binds
  (CharacterBinds|CharacteronTakeRadialDamage DamagedActor Damage DamageType Origin HitInfo InstigatedBy DamageCauser))

(event Custom|ClientSetLocAndRotPlaySpace
  (params (Loc :type Vector) (Yaw :type Float%20%28single-precision%29))
  (Transformation|SetActorLocationAndRotation (Variables|DataReplicated|GetOwningCharacter) Loc (Math|Rotator|MakeRotator 0.0 0.0 Yaw) false true))

(event EventBeginPlay
  (|CallParentFunction)
  (if (Networking|IsServer)
    (if (Utilities|IsValid (Class|PavlovPlayerProxy|GetPawn)) :!label _label
      (Initialization|ServerInitialization)
      (else
        (Utilities|FlowControl|Delay 0.05)
        (goto _label)))))

(event EventOnPlayerDeath
  (params (KilledActor :type Actor%20Object%20Reference))
  (if (Networking|IsServer)
    (Variables|DataReplicated|SetbIsDead true)))

(event EventTick
  (params (DeltaSeconds :type Float%20%28single-precision%29))
  (|CallParentFunction DeltaSeconds)
  (if (Networking|IsServer)
    (Tick|ServerTick DeltaSeconds))
  (if (Default|IsLocalPRI (Variables|DataReplicated|GetOwningPRI))
    (Tick|LocalTick DeltaSeconds)
    (else
      (Tick|RemoteTick DeltaSeconds))))

(fn ConstructionScript
  (|CallParentFunction))

(fn SpawnPlayerOverheadVisual
  (if (Variables|/Game/CustomMaps/UGC1908549791/PMF/Blueprints/LevelActors/CORE/PMF_GameLogic.PMF_GameLogic_C|GetbUsePMFPlayerInfo (CallFunction|GetPMFGameLogic))
    (if (not (Default|IsLocalPRI (Variables|DataReplicated|GetOwningPRI)))
      (Utilities|IsValid (Variables|Data|GetSpawnedPlayerInfo)
        (:Is%20Not%20Valid
          (bind _returnvalue (Game|SpawnActorfromClass (Variables|Config|GetPlayerOverheadVisualClass) (Math|Transform|MakeTransform "0, 0, 0") "AlwaysSpawn" 0 (Variables|DataReplicated|GetOwningPRI) 0))
          (Variables|Data|SetSpawnedPlayerInfo _returnvalue))))))

(fn OnRepBIsDead
  (Utilities|FlowControl|Sequence
    (:then_0
      (Creation|DestroyPlayerOverheadVisual))
    (:then_1
      (if (Default|IsLocalPRI (Variables|DataReplicated|GetOwningPRI))
        (Default|RefreshPlayerInputs (Variables|DataReplicated|GetOwningPRI))))))

(fn DestroyPlayerOverheadVisual
  (Utilities|IsValid (Variables|Data|GetSpawnedPlayerInfo)
    (:Is%20Valid
      (Actor|DestroyActor (Variables|Data|GetSpawnedPlayerInfo)))))

(fn PlayerLeftServer
  (Actor|DestroyActor))

(fn GetOwningPRI
  (bind _owningpri (Variables|DataReplicated|GetOwningPRI))
  (Utilities|IsValid (Variables|DataReplicated|GetOwningPRI)
    (:Is%20Valid
      (return true (Default|IsLocalPRI _owningpri) _owningpri))
    (:Is%20Not%20Valid
      (return false false 0))))

(fn GetOwningCharacter
  (Utilities|IsValid (Variables|DataReplicated|GetOwningCharacter)
    (:Is%20Valid
      (return true (Variables|DataReplicated|GetOwningCharacter)))
    (:Is%20Not%20Valid
      (return false 0))))

(fn GetIsDead
  (return (Variables|DataReplicated|GetbIsDead)))

(fn ServerInitialization
  (bind _playersettings (Variables|Config|GetPlayerSettings))
  (bind _playersettings_2 (Variables|Config|GetPlayerSettings))
  (bind _playersettings_3 (Variables|Config|GetPlayerSettings))
  (bind _playersettings_4 (Variables|Config|GetPlayerSettings))
  (bind _playersettings_5 (Variables|Config|GetPlayerSettings))
  (bind (_health _armour _helmet) (Utilities|Struct|BreakPMF_PlayerSettingsData _playersettings))
  (bind (_cashsetperround _cashaddedperround) (Utilities|Struct|BreakPMF_PlayerSettingsData _playersettings_3))
  (bind (_busedefaultloadout _defaultloadout) (Utilities|Struct|BreakPMF_PlayerSettingsData _playersettings_2))
  (bind (_benablebuying _buyduration _buyzonemaxdistance) (Utilities|Struct|BreakPMF_PlayerSettingsData _playersettings_4))
  (bind _cashongamestart (Utilities|Struct|BreakPMF_PlayerSettingsData _playersettings_5))
  (Utilities|FlowControl|Sequence
    (:then_0
      (bind _ascharacter (Utilities|Casting|CastToCharacter (Class|PavlovPlayerProxy|GetPawn)))
      (Variables|DataReplicated|SetOwningCharacter _ascharacter))
    (:then_1
      (CallFunction|RegisterCharacterDamageEvents))
    (:then_2
      (Utilities|FlowControl|Sequence
        (:then_0
          (if _benablebuying
            (Class|PavlovGameLogic|SetPlayerBuyingEnabled (CallFunction|GetPMFGameLogic) (Default|GetOwningPlayerState (Variables|DataReplicated|GetOwningPRI)) _buyduration _buyzonemaxdistance)
            (if (> _cashsetperround 0) ; Set Cash On Round Start?
              (Class|PavlovGameLogic|SetPlayerCash (CallFunction|GetPMFGameLogic) (Default|GetOwningPlayerState (Variables|DataReplicated|GetOwningPRI)) _cashsetperround)
              (elif (== (Variables|/Game/CustomMaps/UGC1908549791/PMF/Blueprints/LevelActors/CORE/PMF_GameLogic.PMF_GameLogic_C|GetRoundCount (CallFunction|GetPMFGameLogic)) 1)
                (if (> _cashongamestart 0)
                  (Class|PavlovGameLogic|SetPlayerCash (CallFunction|GetPMFGameLogic) (Default|GetOwningPlayerState (Variables|DataReplicated|GetOwningPRI)) _cashongamestart)
                  (else
                    (if (> _cashaddedperround 0) :!label _label
                      (Class|PavlovGameLogic|GivePlayerCash (CallFunction|GetPMFGameLogic) (Default|GetOwningPlayerState (Variables|DataReplicated|GetOwningPRI)) _cashaddedperround))))
                (else
                  (goto _label))))))
        (:then_1
          (Class|PavlovGameLogic|SetPlayerVitality (CallFunction|GetPMFGameLogic) (Default|GetOwningPlayerState (Variables|DataReplicated|GetOwningPRI)) _health _armour _helmet))
        (:then_2
          (if _busedefaultloadout
            (Default|SpawnDefaultLoadOut (CallFunction|GetPMFGameLogic) (Variables|DataReplicated|GetOwningPRI) _defaultloadout)))))
    (:then_3
      (if (Variables|Config|GetbDisableDamage)
        (Variables|/Script/Engine.Actor|SetbCanBeDamaged (Variables|DataReplicated|GetOwningCharacter) false)))
    (:then_4
      (Actor|Tick|SetActorTickEnabled (Variables|Config|GetbTickServer)))))

(fn ClientInitialization
  (bind (_bisvalid _bislocal _owningpri) (Info|GetOwningPRI))
  (if (not (Networking|IsServer))
    (Utilities|FlowControl|Sequence
      (:then_0
        (Creation|SpawnPlayerOverheadVisual))
      (:then_1
        (if (Variables|Config|GetbSkeletonGeneratesOverlapEvents)
          (Character|SetGenerateOverlap true)))
      (:then_2
        (Speed|SetPlayerSpeed (Variables|Config|GetPlayerSpeedMultiplier)))
      (:then_3
        (if _bislocal
          (Default|RefreshInputs (Variables|/Game/CustomMaps/UGC1908549791/PMF/Blueprints/Info/PMF_PlayerReplicationInfo.PMF_PlayerReplicationInfo_C|GetPMFPlayerInput _owningpri))))
      (:then_4
        (Actor|Tick|SetActorTickEnabled (select (Default|IsLocalPRI (Variables|DataReplicated|GetOwningPRI)) (Variables|Config|GetbTickLocal) (Variables|Config|GetbTickRemote)))))))

(fn OnRepOwningCharacter
  (if (not (Networking|IsServer))
    (Initialization|ClientInitialization)))

(fn JumpPlayer
  (Utilities|IsValid (Variables|DataReplicated|GetOwningCharacter)
    (:Is%20Valid
      (if (Pawn|IsLocallyControlled (Variables|DataReplicated|GetOwningCharacter)) ; Only the local player can decide to jump
        (bind _bcanjump (Jumping|CanJump))
        (if _bcanjump
          (Character|LaunchCharacter (Variables|DataReplicated|GetOwningCharacter) (Math|Vector|MakeVector 0.0 0.0 (Variables|Config|GetJumpForce)) false true))))))

(fn CanJump
  (bind _owningcharacter (Variables|DataReplicated|GetOwningCharacter))
  (if (Variables|Config|GetbAllowJumpingEver)
    (Utilities|IsValid _owningcharacter
      (:Is%20Valid
        (if (AI|Components|NavMovement|IsFalling (Variables|/Script/Engine.Character|GetCharacterMovement _owningcharacter)) ; By default anyone grounded can jump
          (return false)
          (else
            (return true))))
      (:Is%20Not%20Valid
        (return false)))
    (else
      (return false))))

(fn LowGravity
  (params (DeltaTime :type Float%20%28single-precision%29))
  (bind _owningcharacter (Variables|DataReplicated|GetOwningCharacter))
  (if (Default|IsLocalPRI (Variables|DataReplicated|GetOwningPRI))
    (if (!= (Variables|Config|GetGravityForce) 0.0) ; Only Apply It If It Isn't Default
      (Utilities|IsValid _owningcharacter
        (:Is%20Valid
          (if (AI|Components|NavMovement|IsFalling (Variables|/Script/Engine.Character|GetCharacterMovement _owningcharacter))
            (CallFunction|AddVelocitytoCharacter _owningcharacter (Math|Vector|MakeVector 0.0 0.0 (* (Variables|Config|GetGravityForce) DeltaTime)))))))))

(fn LimitHorizontalVelocity
  (bind _owningcharacter (Variables|DataReplicated|GetOwningCharacter))
  (bind _horizontalvelocitylimit (Variables|Config|GetHorizontalVelocityLimit))
  (bind _returnvalue (Transformation|GetVelocity _owningcharacter))
  (bind (_x _y _z) (Math|Vector|BreakVector _returnvalue))
  (bind _returnvalue_2 (Math|Vector|MakeVector _x _y 0.0))
  (bind _returnvalue_3 (Math|Vector|ClampVectorSize _returnvalue_2 0.0 _horizontalvelocitylimit))
  (bind (_x_2 _y_2) (Math|Vector|BreakVector _returnvalue_3))
  (if (Default|IsLocalPRI (Variables|DataReplicated|GetOwningPRI))
    (if (!= (Variables|Config|GetHorizontalVelocityLimit) 0.0) ; Only Apply It If It Isn't Default
      (Utilities|IsValid _owningcharacter
        (:Is%20Valid
          (if (AI|Components|NavMovement|IsFalling (Variables|/Script/Engine.Character|GetCharacterMovement _owningcharacter))
            (if (> (Math|Vector|VectorLengthXY _returnvalue) (Variables|Config|GetHorizontalVelocityLimit))
              (Variables|/Script/Engine.MovementComponent|SetVelocity (Pawn|GetMovementComponent (Class|CharacterMovementComponent|GetCharacterOwner (Variables|/Script/Engine.Character|GetCharacterMovement _owningcharacter))) (Math|Vector|MakeVector _x_2 _y_2 _z)))))))))

(fn ServerTick
  (params (DeltaTime :type Float%20%28single-precision%29)))

(fn LocalTick
  (params (DeltaTime :type Float%20%28single-precision%29))
  (Utilities|FlowControl|Sequence
    (:then_0
      (Gravity|LowGravity DeltaTime))
    (:then_1
      (Gravity|LimitHorizontalVelocity))))

(fn RemoteTick
  (params (DeltaTime :type Float%20%28single-precision%29)))

(fn OnRepPlayerSpeedMultiplier
  (Speed|SetPlayerSpeed (Variables|Config|GetPlayerSpeedMultiplier)))

(fn SetPlayerSpeed
  (params (Multiplier :type Float%20%28single-precision%29))
  (bind _owningcharacter (Variables|DataReplicated|GetOwningCharacter))
  (bind _charactermovement (Variables|/Script/Engine.Character|GetCharacterMovement _owningcharacter))
  (Variables|/Script/Engine.CharacterMovementComponent|SetMaxCustomMovementSpeed _charactermovement (* (Variables|/Script/Engine.CharacterMovementComponent|GetMaxCustomMovementSpeed _charactermovement) Multiplier))
  (Variables|/Script/Engine.CharacterMovementComponent|SetMaxWalkSpeed _charactermovement (* (Variables|/Script/Engine.CharacterMovementComponent|GetMaxWalkSpeed _charactermovement) Multiplier))
  (Variables|/Script/Engine.CharacterMovementComponent|SetMaxWalkSpeedCrouched _charactermovement (* (Variables|/Script/Engine.CharacterMovementComponent|GetMaxWalkSpeedCrouched _charactermovement) Multiplier))
  (Variables|/Script/Engine.CharacterMovementComponent|SetMinAnalogWalkSpeed _charactermovement (* (Variables|/Script/Engine.CharacterMovementComponent|GetMinAnalogWalkSpeed _charactermovement) Multiplier)))

(fn CharacteronTakeAnyDamage
  (params (DamagedActor :type Actor%20Object%20Reference) (Damage :type Float%20%28single-precision%29) (DamageType :type Damage%20Type%20Object%20Reference) (InstigatedBy :type Controller%20Object%20Reference) (DamageCauser :type Actor%20Object%20Reference)))

(fn CharacteronTakePointDamage
  (params (DamagedActor :type Actor%20Object%20Reference) (Damage :type Float%20%28single-precision%29) (InstigatedBy :type Controller%20Object%20Reference) (HitLocation :type Vector) (FHitComponent :type Primitive%20Component%20Object%20Reference) (BoneName :type Name) (ShotFromDirection :type Vector) (DamageType :type Damage%20Type%20Object%20Reference) (DamageCauser :type Actor%20Object%20Reference)))

(fn CharacteronTakeRadialDamage
  (params (DamagedActor :type Actor%20Object%20Reference) (Damage :type Float%20%28single-precision%29) (DamageType :type Damage%20Type%20Object%20Reference) (Origin :type Vector) (HitInfo :type Hit%20Result%20Structure) (InstigatedBy :type Controller%20Object%20Reference) (DamageCauser :type Actor%20Object%20Reference)))

(fn SetGenerateOverlap
  (params (bGenerateOverlapEvents :type Boolean))
  (bind _returnvalue (Class|PavlovPlayerProxy|GetPlayerSkeleton))
  (bind _output_get (Variables|/Script/Engine.PrimitiveComponent|SetbGenerateOverlapEvents _returnvalue bGenerateOverlapEvents))
  (Collision|SetCollisionResponsetoChannel _returnvalue "ECC_PhysicsBody" (select _output_get "ECR_Overlap" "ECR_Ignore")))

(fn DropRestrictedItems
  (params (RestrictedItems :type Array%20of%20Names))
  (if (> (Utilities|Array|Length RestrictedItems) 0)
    (bind _items (Class|PavlovPlayerProxy|GetAllItems))
    (for _array_element _items
      (if (Utilities|Array|ContainsItem RestrictedItems (.ItemName (Utilities|Struct|BreakPlayerItem _array_element)))
        (Class|PavlovPlayerProxy|DropItem (.ItemName (Utilities|Struct|BreakPlayerItem _array_element)) false false)))))

(fn KeepRestrictedItemsOnly
  (params (RestrictedItems :type Array%20of%20Names))
  (if (> (Utilities|Array|Length RestrictedItems) 0)
    (bind _items (Class|PavlovPlayerProxy|GetAllItems))
    (for _array_element _items
      (if (not (Utilities|Array|ContainsItem RestrictedItems (.ItemName (Utilities|Struct|BreakPlayerItem _array_element))))
        (Class|PavlovPlayerProxy|DropItem (.ItemName (Utilities|Struct|BreakPlayerItem _array_element)) false false)))))