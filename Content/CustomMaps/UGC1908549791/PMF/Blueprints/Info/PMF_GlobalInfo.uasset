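; PMF global info Blueprint that serves as a lookup between custom item IDs and item classes.
; On BeginPlay it reads the custom item data table and fills two maps, using row names as IDs, for lookups in both directions.
; GetItemIDFromClass and GetItemClassFromID query those maps and return a validity flag.
; The caching pass also iterates the player skin table but stores nothing from it.
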(event EventBeginPlay
  (CallFunction|CacheDataTables))

(event EventTick
  (params (DeltaSeconds :type Float%20%28single-precision%29)))

(fn CacheDataTables
  (Utilities|FlowControl|Sequence
    (:then_0
      (bind _outrownames (DataTable|GetDataTableRowNames (Variables|Default|GetCustomItemTable)))
      (for _array_element _outrownames
        (bind _returnvalue (Utilities|GetDataTableRow (Variables|Default|GetCustomItemTable) _array_element)
          (:then
            (Utilities|Map|Add (Variables|Default|GetIDToItemClass) _array_element (Utilities|Struct|BreakCustomItemData _returnvalue))
            (Utilities|Map|Add (Variables|Default|GetItemClassToID) (Utilities|Struct|BreakCustomItemData _returnvalue) _array_element)))))
    (:then_1
      (bind _outrownames_2 (DataTable|GetDataTableRowNames (Variables|Default|GetPlayerSkinTable)))
      (for _array_element_2 _outrownames_2
        (bind _returnvalue_2 (Utilities|GetDataTableRow (Variables|Default|GetPlayerSkinTable) _array_element_2))))))

(fn GetItemIDfromClass
  (params (ItemClass :type Pavlov%20Custom%20Item%20Class%20Reference))
  (bind _itemclasstoid (Variables|Default|GetItemClassToID))
  (bind (_value _returnvalue) (Utilities|Map|Find _itemclasstoid ItemClass))
  (return _value _returnvalue))

(fn GetItemClassfromID
  (params (ItemID :type Name))
  (bind _idtoitemclass (Variables|Default|GetIDToItemClass))
  (bind (_value _returnvalue) (Utilities|Map|Find _idtoitemclass ItemID))
  (return _value _returnvalue))