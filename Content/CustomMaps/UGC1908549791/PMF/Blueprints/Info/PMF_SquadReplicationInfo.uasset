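; PMF squad replication info that holds one squad's name, score, wins, lock state, member player infos (PRIs) and leader.
; Simple getters and setters expose score and wins, and queries report player count, living members, leadership and free slots against the game logic's max squad size.
; Locking, leader promotion and kicking are server-only, with promote and kick validating squad membership.
; PlayerJoinSquad and PlayerLeaveSquad are empty here, so kicking only calls that stub.
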(event EventBeginPlay)

(event Collision|EventActorBeginOverlap
  (params (OtherActor :type Actor%20Object%20Reference)))

(event EventTick
  (params (DeltaSeconds :type Float%20%28single-precision%29)))

(fn ConstructionScript)

(fn SetSquadScore
  (params (NewScore :type Integer))
  (Variables|DataReplicated|SetSquadScore NewScore))

(fn SetSquadWins
  (params (NewWins :type Integer))
  (Variables|DataReplicated|SetSquadWins NewWins))

(fn AddSquadScore
  (params (AdditionalScore :type Integer))
  (Variables|DataReplicated|SetSquadScore (+ AdditionalScore (Variables|DataReplicated|GetSquadScore))))

(fn IncrementSquadScore
  (Math|Integer|IncrementInt (Variables|DataReplicated|GetSquadScore)))

(fn IncrementSquadWins
  (Math|Integer|IncrementInt (Variables|DataReplicated|GetSquadWins)))

(fn GetPlayerCount
  (return (Utilities|Array|Length (Variables|DataReplicated|GetSquadPRIs))))

(fn GetSquadScore
  (return (Variables|DataReplicated|GetSquadScore)))

(fn GetSquadWins
  (return (Variables|DataReplicated|GetSquadWins)))

(fn GetSquadName
  (return (Variables|DataReplicated|GetSquadName)))

(fn IsSquadLocked
  (return (Variables|DataReplicated|GetbSquadIsLocked)))

(fn GetSquadLeaderPRI
  (return (Variables|DataReplicated|GetSquadLeaderPRI)))

(fn PlayerJoinSquad
  (params (PRI :type PMF%20Player%20Replication%20Info%20Object%20Reference)))

(fn PlayerLeaveSquad
  (params (PRI :type PMF%20Player%20Replication%20Info%20Object%20Reference)))

(fn LockSquad
  (if (Networking|IsServer)
    (Variables|DataReplicated|SetbSquadIsLocked true)))

(fn UnlockSquad
  (if (Networking|IsServer)
    (Variables|DataReplicated|SetbSquadIsLocked false)))

(fn ToggleSquadLock
  (if (Networking|IsServer)
    (if (Getters|IsSquadLocked)
      (Locking|UnlockSquad)
      (else
        (Locking|LockSquad)))))

(fn PromoteSquadLeader
  (params (PRI :type PMF%20Player%20Replication%20Info%20Object%20Reference))
  (if (Networking|IsServer)
    (Utilities|IsValid PRI
      (:Is%20Valid
        (if (!= PRI (Variables|DataReplicated|GetSquadLeaderPRI))
          (if (== (Variables|DataReplicated|GetSquadIndex) (Default|GetSquadIndex PRI))
            (if (Utilities|Array|ContainsItem (Variables|DataReplicated|GetSquadPRIs) PRI)
              (Variables|DataReplicated|SetSquadLeaderPRI PRI))))))))

(fn KickfromSquad
  (params (PRI :type PMF%20Player%20Replication%20Info%20Object%20Reference))
  (if (Networking|IsServer)
    (Utilities|IsValid PRI
      (:Is%20Valid
        (if (!= PRI (Variables|DataReplicated|GetSquadLeaderPRI))
          (if (== (Variables|DataReplicated|GetSquadIndex) (Default|GetSquadIndex PRI))
            (if (Utilities|Array|ContainsItem (Variables|DataReplicated|GetSquadPRIs) PRI)
              (Joining|PlayerLeaveSquad PRI))))))))

(fn HasAnyPlayers
  (return (> (Getters|GetPlayerCount) 0)))

(fn HasAlivePlayers
  (for _array_element (Variables|DataReplicated|GetSquadPRIs)
    (if (not (Default|IsDead _array_element))
      (return true)))
  (return false))

(fn IsSquadLeader
  (params (PRI :type PMF%20Player%20Replication%20Info%20Object%20Reference))
  (return (and (Utilities|IsValid (Variables|DataReplicated|GetSquadLeaderPRI)) (== (Variables|DataReplicated|GetSquadLeaderPRI) PRI))))

(fn GetSlotsLeft
  (return (- (Variables|/Game/CustomMaps/UGC1908549791/PMF/Blueprints/LevelActors/CORE/PMF_GameLogic.PMF_GameLogic_C|GetMaxSquadSize (CallFunction|GetPMFGameLogic)) (Getters|GetPlayerCount))))

(fn HasSlotsLeft
  (return (> (Info|GetSlotsLeft) 0)))