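; PMF_CooldownComp is a cooldown component that tracks whether something can be used again.
; Used stamps LastTimeUsed with the GameState's server world time, and Reset restores that value to the class default.
; CanUse compares that stamp plus CooldownDuration to current server time, so no timer or tick is involved.
; Helper functions derive the remaining time, the clamped fraction remaining and the finish time from the same values.
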(fn Used
  (Variables|Data|SetLastTimeUsed (GameState|GetServerWorldTimeSeconds (Game|GetGameState))))

(fn Reset
  (Variables|Data|SetLastTimeUsed (.LastTimeUsed (Utilities|GetClassDefaults "PMF_CooldownComp_C"))))

(fn CanUse
  (return (< (+ (Variables|Config|GetCooldownDuration) (Variables|Data|GetLastTimeUsed)) (GameState|GetServerWorldTimeSeconds (Game|GetGameState)))))

(fn GetRemainingTime
  (if (CallFunction|CanUse)
    (return 0.0)
    (else
      (return (- (+ (Variables|Config|GetCooldownDuration) (Variables|Data|GetLastTimeUsed)) (GameState|GetServerWorldTimeSeconds (Game|GetGameState)))))))

(fn GetCooldownPercent
  (return (Math|Float|Clamp(Float) (/ (CallFunction|GetRemainingTime) (Variables|Config|GetCooldownDuration)))))

(fn GetFinishTime
  (if (CallFunction|CanUse)
    (return (GameState|GetServerWorldTimeSeconds (Game|GetGameState)))
    (else
      (return (+ (Variables|Config|GetCooldownDuration) (Variables|Data|GetLastTimeUsed))))))