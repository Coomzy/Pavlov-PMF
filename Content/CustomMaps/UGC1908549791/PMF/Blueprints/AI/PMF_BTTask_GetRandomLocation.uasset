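; Behavior tree task that picks a random nearby location around a stored start point for an AI.
; On execute it flattens a random unit vector to the horizontal plane, scales it by a small random distance and adds it to the start location from the blackboard.
; The result is written to the new-location blackboard key, with no navmesh check and no FinishExecute call in the graph.
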(event EventReceiveExecute
  (params (OwnerActor :type Actor%20Object%20Reference))
  (bind _returnvalue (AI|GetBlackboard OwnerActor))
  (bind _returnvalue_2 (Math|Random|RandomUnitVector))
  (bind (_x _y) (Math|Vector|BreakVector _returnvalue_2))
  (AI|Components|Blackboard|SetValueasVector _returnvalue (Variables|Default|GetBB_Key_NewLoc) (+ (AI|Components|Blackboard|GetValueasVector _returnvalue (Variables|Default|GetBB_Key_StartLoc)) (* (Math|Vector|Normalize (Math|Vector|MakeVector _x _y 0.0)) (Math|Random|RandomFloatinRange 1.0 1e+01)))))