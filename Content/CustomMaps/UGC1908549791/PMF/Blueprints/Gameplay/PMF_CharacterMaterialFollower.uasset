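; Follower actor that overlays a material on a Pavlov character by mirroring its body and helmet meshes.
; Each copier attaches to the source mesh, takes its skeletal mesh, swaps every material to MaterialToApply and follows via master pose.
; By default it applies to the PRI's character and destroys itself when the PRI dies or becomes invalid.
; With AllowNonPRIUse, it instead hides whenever the applied character was recently rendered.
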(event Custom|ApplyMaterialTo
  (params (Char :type Character%20Object%20Reference))
  (bind _returnvalue (Actor|GetComponentsByClass Char "/Script/Engine.SkeletalMeshComponent"))
  (bind _indexs (CallFunction|GetPavlovIndexs))
  (Variables|Default|SetAppliedChar Char)
  (CallFunction|CopySkeletalMesh (Variables|Default|GetPlayerBodyEffect) (Utilities|Array|Get(acopy) _returnvalue (Variables|/Game/CustomMaps/UGC1908549791/PMF/Blueprints/Data/Objects/PMF_PavlovIndexs.PMF_PavlovIndexs_C|GetInventoryCharacterBodyMeshOffset _indexs)))
  (CallFunction|CopySkeletalMesh (Variables|Default|GetPlayerHelmetEffect) (Utilities|Array|Get(acopy) _returnvalue (Variables|/Game/CustomMaps/UGC1908549791/PMF/Blueprints/Data/Objects/PMF_PavlovIndexs.PMF_PavlovIndexs_C|GetInventoryCharacterHelmetMeshOffset _indexs))))

(event EventBeginPlay
  (bind _pri (Variables|Default|GetPRI))
  (if (not (Variables|Default|GetbAllowNonPRIUse))
    (Utilities|IsValid _pri
      (:Is%20Valid
        (CallFunction|ApplyMaterialto (.Character (Default|GetPlayerCharacter _pri)))))))

(event EventTick
  (params (DeltaSeconds :type Float%20%28single-precision%29))
  (if (Variables|Default|GetbAllowNonPRIUse)
    (Utilities|IsValid (Variables|Default|GetAppliedChar)
      (:Is%20Valid
        (Rendering|SetActorHiddenInGame (Class|Actor|WasRecentlyRendered (Variables|Default|GetAppliedChar) 0.01))))
    (else
      (Utilities|IsValid (Variables|Default|GetPRI)
        (:Is%20Valid
          (if (not (Game|IsActorBeingDestroyed))
            (if (Default|IsDead (Variables|Default|GetPRI))
              (Actor|DestroyActor :!label _label))))
        (:Is%20Not%20Valid
          (goto _label))))))

(fn ConstructionScript)

(fn CopySkeletalMesh
  (params (SkeletalMeshCopier :type Skeletal%20Mesh%20Component%20Object%20Reference) (SkeletalMeshToCopy :type Skeletal%20Mesh%20Component%20Object%20Reference))
  (Utilities|IsValid SkeletalMeshCopier
    (:Is%20Valid
      (Utilities|IsValid SkeletalMeshToCopy
        (:Is%20Valid
          (Transformation|AttachComponentToComponent SkeletalMeshCopier SkeletalMeshToCopy "None" "SnapToTarget" "SnapToTarget" "SnapToTarget" true)
          (Class|SkinnedMeshComponent|SetSkeletalMesh SkeletalMeshCopier (Variables|/Script/Engine.SkinnedMeshComponent|GetSkeletalMesh SkeletalMeshToCopy) false)
          (for (_ _array_index) (Rendering|Material|GetMaterials SkeletalMeshCopier)
            (Rendering|Material|SetMaterial SkeletalMeshCopier _array_index (Variables|Default|GetMaterialToApply)))
          (Class|SkinnedMeshComponent|SetMasterPoseComponent SkeletalMeshCopier SkeletalMeshToCopy true))))))