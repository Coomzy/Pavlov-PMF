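; PMF_Volume_Player is a base trigger volume that detects player pawns entering and leaving a collision box.
; Overlaps are filtered by a VolumeMode setting that combines server, client, local and remote rules using server and local-control checks.
; Valid pawns have their PRI looked up through PMF game logic and passed to empty OnPlayerEnter and OnPlayerExit hooks.
; Helper functions report whether the mode allows server or client execution, but the overlap events do not call them.
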(event OnComponentBeginOverlap(PlayerCollisionBox)
  (params (OverlappedComponent :type Primitive%20Component%20Object%20Reference) (OtherActor :type Actor%20Object%20Reference) (OtherComp :type Primitive%20Component%20Object%20Reference) (OtherBodyIndex :type Integer) (bFromSweep :type Boolean) (SweepResult :type Hit%20Result%20Structure%20%28by%20ref%29))
  (bind _aspawn (Utilities|Casting|CastToPawn OtherActor))
  (bind _bisvalid (CallFunction|IsPawnValidforVolumeMode _aspawn))
  (if _bisvalid
    (bind _outpri (Default|GetPRIbyPlayerState (CallFunction|GetPMFGameLogic) (Variables|/Script/Engine.Pawn|GetPlayerState _aspawn)))
    (CallFunction|OnPlayerEnter _outpri _aspawn)))

(event OnComponentEndOverlap(PlayerCollisionBox)
  (params (OverlappedComponent :type Primitive%20Component%20Object%20Reference) (OtherActor :type Actor%20Object%20Reference) (OtherComp :type Primitive%20Component%20Object%20Reference) (OtherBodyIndex :type Integer))
  (bind _aspawn (Utilities|Casting|CastToPawn OtherActor))
  (bind _bisvalid (CallFunction|IsPawnValidforVolumeMode _aspawn))
  (if _bisvalid
    (bind _outpri (Default|GetPRIbyPlayerState (CallFunction|GetPMFGameLogic) (Variables|/Script/Engine.Pawn|GetPlayerState _aspawn)))
    (CallFunction|OnPlayerExit _outpri _aspawn)))

(fn ConstructionScript)

(fn OnPlayerEnter
  (params (PRI :type PMF%20Player%20Replication%20Info%20Object%20Reference) (Pawn :type Pawn%20Object%20Reference)))

(fn OnPlayerExit
  (params (PRi :type PMF%20Player%20Replication%20Info%20Object%20Reference) (Pawn :type Pawn%20Object%20Reference)))

(fn IsVolumeAllowedonServer
  (bind _volumemode (Variables|Config|GetVolumeMode))
  (return (Math|Boolean|ORBoolean (Utilities|Enum|Equal(Enum) _volumemode "NewEnumerator0") (Utilities|Enum|Equal(Enum) _volumemode "NewEnumerator3") (Utilities|Enum|Equal(Enum) _volumemode "NewEnumerator4") (Utilities|Enum|Equal(Enum) _volumemode "NewEnumerator5"))))

(fn IsVolumeAllowedonClient
  (return (Utilities|Enum|NotEqual(Enum) (Variables|Config|GetVolumeMode) "NewEnumerator3")))

(fn IsPawnValidforVolumeMode
  (params (Pawn :type Pawn%20Object%20Reference))
  (Utilities|IsValid Pawn
    (:Is%20Valid
      (switch Utilities|FlowControl|Switch|SwitchonEPMF_VolumeMode (Variables|Config|GetVolumeMode)
        (:NewEnumerator0
          (return true))
        (:NewEnumerator1
          (return true))
        (:NewEnumerator2
          (return (Pawn|IsLocallyControlled Pawn)))
        (:NewEnumerator6
          (return (not (Pawn|IsLocallyControlled Pawn))))
        (:NewEnumerator3
          (return true))
        (:NewEnumerator4
          (return (or (Networking|IsServer) (Pawn|IsLocallyControlled Pawn))))
        (:NewEnumerator5
          (return (or (Networking|IsServer) (not (Pawn|IsLocallyControlled Pawn)))))))
    (:Is%20Not%20Valid
      (return false))))