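; Last Man Standing marker actor for what appears to be an Infection game mode, bound to a player through its owning player replication info.
; On BeginPlay, the server snap-attaches it to that player's pawn.
; Each server tick, it destroys itself once the player is dead or the owning info becomes invalid.
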(event EventBeginPlay
  (if (Networking|IsServer)
    (Transformation|AttachActorToActor (.Pawn (Default|GetPlayerPawn (Variables|Default|GetOwningPRI))) "None" "SnapToTarget" "SnapToTarget" "SnapToTarget" true)))

(event EventTick
  (params (DeltaSeconds :type Float%20%28single-precision%29))
  (if (Networking|IsServer)
    (if (not (Game|IsActorBeingDestroyed))
      (Utilities|IsValid (Variables|Default|GetOwningPRI)
        (:Is%20Valid
          (if (Default|IsDead (Variables|Default|GetOwningPRI))
            (Actor|DestroyActor)))
        (:Is%20Not%20Valid
          (Actor|DestroyActor))))))

(fn ConstructionScript)