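; Player replication info for the Infection mode, tracking whether a player is a zombie by team index and whether they are an alpha zombie.
; Becoming alpha plays an infected announcement, and local client initialization plays the infection announcement.
; When the game award system is on, kills trigger killing-spree and timed multi-kill checks that queue award sounds from lookup maps.
; It also spawns the game logic's Last Man Standing actor for its player.
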(event EventAddKills
  (Variables|Data|SetCachedLastKillTime (Variables|Default|GetLastKillTime))
  (|CallParentFunction)
  (if (Variables|/Game/CustomMaps/UGC1908549791/INF/Blueprints/LevelActors/CORE/INF_GameLogic.INF_GameLogic_C|GetbUseGameAwardSystem (CallFunction|GetINFGameLogic))
    (CallFunction|CheckKillingSpree)
    (CallFunction|CheckMultiKill (Variables|Data|GetCachedLastKillTime))))

(event EventClientInitialization
  (|CallParentFunction)
  (if (CallFunction|IsLocalPRI)
    (Default|PlayInfectionAnnouncement (.AsINF%20Sound%20Manager (CallFunction|GetINFSoundManager)))))

(fn ConstructionScript
  (|CallParentFunction))

(fn IsZombie
  (return (== (CallFunction|GetTeamIndex) (Variables|/Game/CustomMaps/UGC1908549791/INF/Blueprints/Data/Objects/INF_GlobalVariables.INF_GlobalVariables_C|GetTeamZombieIndex (CallFunction|GetINFGlobals))) (Variables|DataReplicated|GetbIsAlphaZombie)))

(fn BecomeAlphaZombie
  (Variables|DataReplicated|SetbIsAlphaZombie true)
  (Default|PlayInfectedAnnouncement (.AsINF%20Sound%20Manager (CallFunction|GetINFSoundManager)) self))

(fn BecomeHuman
  (Variables|DataReplicated|SetbIsAlphaZombie false))

(fn ApplyLastManStanding
  (Game|SpawnActorfromClass (Variables|/Game/CustomMaps/UGC1908549791/INF/Blueprints/LevelActors/CORE/INF_GameLogic.INF_GameLogic_C|GetLastManStandingActorClass (CallFunction|GetINFGameLogic)) (Math|Transform|MakeTransform "0, 0, 0") "AlwaysSpawn" (CallFunction|GetPlayerController) self 0))

(fn CheckKillingSpree
  (if (not (not (CallFunction|IsDead)))
    (if (Utilities|Map|Contains (Variables|Config-INF|GetKillingSpreeAwards) (Variables|Default|GetKillsThisLife))
      (Default|PlayQueuedSoundforPRI (.PMFSoundManager (CallFunction|GetPMFSoundManager)) self (.Value (Utilities|Map|Find (Variables|Config-INF|GetKillingSpreeAwards) (Variables|Default|GetKillsThisLife))) true))))

(fn CheckMultiKill
  (params (ActualLastKillTime :type Float%20%28single-precision%29))
  (if (<= (- (GameState|GetServerWorldTimeSeconds (Game|GetGameState)) ActualLastKillTime) (Variables|Config-INF|GetMultiKillTimeGap))
    (Math|Integer|IncrementInt (Variables|Data|GetMultiKillCount)
      (:%20%20
        (if (Utilities|Map|Contains (Variables|Config-INF|GetMultiKillAwards) (Variables|Data|GetMultiKillCount))
          (Default|PlayQueuedSoundforPRI (.PMFSoundManager (CallFunction|GetPMFSoundManager)) self (.Value (Utilities|Map|Find (Variables|Config-INF|GetMultiKillAwards) (Variables|Data|GetMultiKillCount))) true))))
    (else
      (Variables|Data|SetMultiKillCount 1))))