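; Player proxy for zombies in the INF mode that restricts them to a forced loadout item and lets them jump.
; Pressing either trigger while that hand holds no item makes the player jump.
; On a 0.1-second server tick it keeps only the forced item and, if missing, respawns it through the PMF game logic into an inventory slot picked by handedness.
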(event EventServerTick
  (params (DeltaTime :type Float%20%28single-precision%29))
  (bind _forceditemsnames (Variables|Data|GetForcedItemsNames))
  (|CallParentFunction DeltaTime)
  (Utilities|FlowControl|Sequence
    (:then_0
      (if (> (Utilities|Array|Length _forceditemsnames) 0)
        (CallFunction|KeepRestrictedItemsOnly _forceditemsnames)))
    (:then_1
      (if (Utilities|Name|NotEqual(Name) (CallFunction|GetItemIDNamebyLoadoutData (Variables|Config|GetForcedItems)) "None")
        (bind _bhasitem (Class|PavlovPlayerProxy|HasItem (CallFunction|GetItemIDNamebyLoadoutData (Variables|Config|GetForcedItems))))
        (if (not _bhasitem)
          (Default|SpawnItemonPlayer (CallFunction|GetPMFGameLogic) (Variables|Default|GetOwningPRI) (Variables|Config|GetForcedItems) true true (select (Default|IsRightHanded (Variables|Default|GetOwningPRI)) 1 0)))))))

(event EventServerInitialization
  (|CallParentFunction)
  (Utilities|FlowControl|Sequence
    (:then_0
      (Actor|Tick|SetActorTickInterval 0.1))
    (:then_1
      (Utilities|Array|AddUnique (Variables|Data|GetForcedItemsNames) (CallFunction|GetItemIDNamebyLoadoutData (Variables|Config|GetForcedItems))))))

(event Input|ActionEvents|InputActionTriggerLeft
  (params (Key :type Key%20Structure))
  (:Pressed
    (bind _bhasitem (Class|PavlovPlayerProxy|GetHeldItem (not (Default|IsRightHanded (.OwningPRI (CallFunction|GetOwningPRI))))))
    (if (not _bhasitem)
      (CallFunction|JumpPlayer))))

(event Input|ActionEvents|InputActionTriggerRight
  (params (Key :type Key%20Structure))
  (:Pressed
    (bind _bhasitem (Class|PavlovPlayerProxy|GetHeldItem (Default|IsRightHanded (.OwningPRI (CallFunction|GetOwningPRI)))))
    (if (not _bhasitem)
      (CallFunction|JumpPlayer))))

(fn ConstructionScript
  (|CallParentFunction))