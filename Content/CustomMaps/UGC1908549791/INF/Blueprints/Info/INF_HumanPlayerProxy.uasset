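; INF_HumanPlayerProxy is a human player proxy for a custom map that lets the player jump with the controller triggers.
; Each left or right trigger press maps to a held-item slot using the owning PRI's handedness setting.
; If that hand holds no item, the press calls JumpPlayer.
; The construction script only runs the parent's.
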(event Input|ActionEvents|InputActionTriggerLeft
  (params (Key :type Key%20Structure))
  (:Pressed
    (bind _bhasitem (Class|PavlovPlayerProxy|GetHeldItem (not (Default|IsRightHanded (.OwningPRI (CallFunction|GetOwningPRI))))))
    (if (not _bhasitem)
      (CallFunction|JumpPlayer))))

(event Input|ActionEvents|InputActionTriggerRight
  (params (Key :type Key%20Structure))
  (:Pressed
    (bind _bhasitem (Class|PavlovPlayerProxy|GetHeldItem (Default|IsRightHanded (.OwningPRI (CallFunction|GetOwningPRI)))))
    (if (not _bhasitem)
      (CallFunction|JumpPlayer))))

(fn ConstructionScript
  (|CallParentFunction))