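; A debug level actor that turns its mesh into a physics ragdoll when it takes any damage.
; The damage event sets a RepNotify flag, whose OnRep switches on physics simulation and collision so the ragdoll state replicates.
; An optional toggle also plays an attenuated Roblox "oof" sound at the mesh location on each hit.
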(event Game|Damage|EventAnyDamage
  (params (Damage :type Float%20%28single-precision%29) (DamageType :type Damage%20Type%20Object%20Reference) (InstigatedBy :type Controller%20Object%20Reference) (DamageCauser :type Actor%20Object%20Reference))
  (Variables|Default|SetbRagdollMesh true)
  (if (Variables|Default|GetbOofOnHit)
    (Audio|PlaySoundatLocation "/Game/CustomMaps/UGC1908549791/DebugPavlov/Audio/Roblox_Death_Sound_-_OOF__Sound_Effect.Roblox_Death_Sound_-_OOF__Sound_Effect" (Transformation|GetWorldLocation (Variables|Character|GetMesh)) "0, 0, 0" 1.0 1.0 0.0 "/Game/CustomMaps/UGC1908549791/DebugPavlov/Audio/Attn_Oof.Attn_Oof" 0 0)))

(fn ConstructionScript)

(fn OnRepBRagdollMesh
  (Physics|SetSimulatePhysics (Variables|Character|GetMesh) true)
  (Collision|SetCollisionObjectType (Variables|Character|GetMesh) "ECC_PhysicsBody")
  (Collision|SetCollisionResponsetoChannel (Variables|Character|GetMesh) "ECC_WorldStatic" "ECR_Block")
  (Collision|SetCollisionEnabled (Variables|Character|GetMesh) "QueryAndPhysics"))