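; DP_CharacterLauncher is a debug-map level actor that launches characters upward when they step into its trigger box.
; On box overlap, a locally controlled Character gets LaunchCharacter with a vertical LaunchForce, overriding Z velocity while keeping XY.
; On BeginPlay it registers itself with its DP_UI_CharacterLauncher widget component as the owning launcher.
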(event OnComponentBeginOverlap(Box)
  (params (OverlappedComponent :type Primitive%20Component%20Object%20Reference) (OtherActor :type Actor%20Object%20Reference) (OtherComp :type Primitive%20Component%20Object%20Reference) (OtherBodyIndex :type Integer) (bFromSweep :type Boolean) (SweepResult :type Hit%20Result%20Structure%20%28by%20ref%29))
  (bind _ascharacter (Utilities|Casting|CastToCharacter OtherActor))
  (if (Pawn|IsLocallyControlled _ascharacter)
    (Character|LaunchCharacter _ascharacter (Math|Vector|MakeVector 0.0 0.0 (Variables|Default|GetLaunchForce)) false true)))

(event EventBeginPlay
  (|CallParentFunction)
  (bind _asdp_ui_character_launcher (Utilities|Casting|CastToDP_UI_CharacterLauncher (UserInterface|GetUserWidgetObject (Variables|Default|GetWidget))))
  (Variables|/Game/CustomMaps/UGC1908549791/DebugPavlov/Blueprints/UMG/DP_UI_CharacterLauncher.DP_UI_CharacterLauncher_C|SetOwningCharacterLauncher _asdp_ui_character_launcher self))

(fn ConstructionScript)