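; DP_CharacterLift is a level actor that pushes locally controlled characters upward while they overlap its box volume.
; Each tick it adds ForceZ scaled by delta time to their Z velocity, skipping anyone already rising faster than MaxVelZ.
; Entering the box gives a small launch, apparently to get them moving.
; On BeginPlay it registers itself with two in-world widgets for ForceZ and MaxVelZ.
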(event OnComponentBeginOverlap(Box)
  (params (OverlappedComponent :type Primitive%20Component%20Object%20Reference) (OtherActor :type Actor%20Object%20Reference) (OtherComp :type Primitive%20Component%20Object%20Reference) (OtherBodyIndex :type Integer) (bFromSweep :type Boolean) (SweepResult :type Hit%20Result%20Structure%20%28by%20ref%29))
  (bind _ascharacter (Utilities|Casting|CastToCharacter OtherActor))
  (if (Pawn|IsLocallyControlled _ascharacter)
    (Character|LaunchCharacter _ascharacter "0, 0,5.000000" false false) ; A little launch might get us going?
  ))

(event EventBeginPlay
  (|CallParentFunction)
  (Utilities|FlowControl|Sequence
    (:then_0
      (bind _asdp_ui_character_lift_force_z (Utilities|Casting|CastToDP_UI_CharacterLift_ForceZ (UserInterface|GetUserWidgetObject (Variables|Default|GetWidgetForceZ))))
      (Variables|/Game/CustomMaps/UGC1908549791/DebugPavlov/Blueprints/UMG/DP_UI_CharacterLift_ForceZ.DP_UI_CharacterLift_ForceZ_C|SetOwningCharacterLift _asdp_ui_character_lift_force_z self))
    (:then_1
      (bind _asdp_ui_character_lift_max_vel_z (Utilities|Casting|CastToDP_UI_CharacterLift_MaxVelZ (UserInterface|GetUserWidgetObject (Variables|Default|GetWidgetMaxVelZ))))
      (Variables|/Game/CustomMaps/UGC1908549791/DebugPavlov/Blueprints/UMG/DP_UI_CharacterLift_MaxVelZ.DP_UI_CharacterLift_MaxVelZ_C|SetOwningCharacterLift _asdp_ui_character_lift_max_vel_z self))))

(event EventTick
  (params (DeltaSeconds :type Float%20%28single-precision%29))
  (for _array_element (Collision|GetOverlappingActors (Variables|Default|GetBox) "/Script/Engine.Character" :!class /Script/Engine.PrimitiveComponent)
    (if (<= (.Z (Math|Vector|BreakVector (Transformation|GetVelocity _array_element))) (Variables|Default|GetMaxVelZ))
      (bind _ascharacter (Utilities|Casting|CastToCharacter _array_element))
      (if (Pawn|IsLocallyControlled _ascharacter)
        (Variables|/Script/Engine.MovementComponent|SetVelocity (Variables|/Script/Engine.Character|GetCharacterMovement _ascharacter) (+ (Math|Vector|MakeVector 0.0 0.0 (* DeltaSeconds (Variables|Default|GetForceZ))) (Variables|/Script/Engine.MovementComponent|GetVelocity (Variables|/Script/Engine.Character|GetCharacterMovement _ascharacter))))))))

(fn ConstructionScript)