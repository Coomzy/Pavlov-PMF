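; Trigger volume actor for a Pavlov custom map that changes a player's team when their character walks into it.
; On server-side box overlap it casts to Character, picks the new team and passes it to the game logic's SetPlayerTeam.
; The team is either toggled from the player's current one or fixed to red or the other team, depending on two flags.
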(event OnComponentBeginOverlap(Box)
  (params (OverlappedComponent :type Primitive%20Component%20Object%20Reference) (OtherActor :type Actor%20Object%20Reference) (OtherComp :type Primitive%20Component%20Object%20Reference) (OtherBodyIndex :type Integer) (bFromSweep :type Boolean) (SweepResult :type Hit%20Result%20Structure%20%28by%20ref%29))
  (if (Networking|IsServer)
    (bind _ascharacter (Utilities|Casting|CastToCharacter OtherActor))
    (bind _teamid (CallFunction|GetNewTeamfor (Variables|/Script/Engine.Pawn|GetPlayerState _ascharacter)))
    (Class|PavlovGameLogic|SetPlayerTeam (Class|PavlovLibrary|GetGameLogic) (Variables|/Script/Engine.Pawn|GetPlayerState _ascharacter) _teamid)))

(fn ConstructionScript)

(fn GetNewTeamfor
  (params (PlayerState :type Player%20State%20Object%20Reference))
  (if (Variables|Default|GetbTogglesTeam)
    (bind _playerstatus (Class|PavlovProxyStatics|GetPavlovPlayerStatus PlayerState))
    (if (== (Utilities|Struct|BreakPavlovPlayerStatus _playerstatus) 0)
      (return 1)
      (else
        (return 0)))
    (elif (Variables|Default|GetbIsRedTeam)
      (return 1)
      (else
        (return 0)))))