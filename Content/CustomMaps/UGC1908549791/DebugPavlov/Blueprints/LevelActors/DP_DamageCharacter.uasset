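; Debug target character that records incoming damage and reacts with hit animations and an "OOF" sound.
; Any, point and radial damage events copy their details as strings into replicated structs, with point and radial also playing the sound at the impact.
; Any damage also updates replicated hit count, total and server time, whose RepNotify plays a random reaction and sound.
; ResetHitData clears those totals.
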(event Game|Damage|EventAnyDamage
  (params (Damage :type Float%20%28single-precision%29) (DamageType :type Damage%20Type%20Object%20Reference) (InstigatedBy :type Controller%20Object%20Reference) (DamageCauser :type Actor%20Object%20Reference))
  (bind _hitdatareplicated (Variables|Default|GetHitDataReplicated))
  (bind (_totaltimeshit _totaldamage) (Utilities|Struct|BreakDP_HitData _hitdatareplicated))
  (Utilities|Struct|SetmembersinDP_AnyDamageData (Variables|Default|GetAnyDamageReplicated) (Utilities|String|ToString(Float) Damage) (Utilities|GetDisplayName DamageType) (Utilities|GetDisplayName InstigatedBy) (Utilities|GetDisplayName DamageCauser) (Utilities|GetDisplayName (Components|GetOwner DamageCauser)))
  (Utilities|Struct|SetmembersinDP_HitData _hitdatareplicated (+ _totaltimeshit 1) (+ _totaldamage Damage) (GameState|GetServerWorldTimeSeconds (Game|GetGameState))))

(event Game|Damage|EventPointDamage
  (params (Damage :type Float%20%28single-precision%29) (DamageType :type Damage%20Type%20Object%20Reference) (HitLocation :type Vector :default "0, 0, 0") (HitNormal :type Vector :default "0, 0, 0") (HitComponent :type Primitive%20Component%20Object%20Reference) (BoneName :type Name :default "None") (ShotFromDirection :type Vector :default "0, 0, 0") (InstigatedBy :type Controller%20Object%20Reference) (DamageCauser :type Actor%20Object%20Reference) (HitInfo :type Hit%20Result%20Structure%20%28by%20ref%29))
  (Utilities|Struct|SetmembersinDP_PointDamageData (Variables|Default|GetPointDamageReplicated) (Utilities|String|ToString(Float) Damage) (Utilities|GetDisplayName DamageType) (Utilities|GetDisplayName InstigatedBy) (Utilities|GetDisplayName DamageCauser) (Utilities|GetDisplayName (Components|GetOwner DamageCauser)) (Utilities|String|ToString(Vector) HitLocation) (Utilities|String|ToString(Vector) HitNormal) (Utilities|GetDisplayName HitComponent) (Utilities|String|ToString(Name) BoneName) (Utilities|String|ToString(Vector) ShotFromDirection))
  (Audio|PlaySoundatLocation "/Game/CustomMaps/UGC1908549791/DebugPavlov/Audio/Roblox_Death_Sound_-_OOF__Sound_Effect.Roblox_Death_Sound_-_OOF__Sound_Effect" HitLocation "0, 0, 0" 1.0 1.0 0.0 "/Game/CustomMaps/UGC1908549791/DebugPavlov/Audio/Attn_Oof.Attn_Oof" 0 0))

(event Game|Damage|EventRadialDamage
  (params (DamageReceived :type Float%20%28single-precision%29) (DamageType :type Damage%20Type%20Object%20Reference) (Origin :type Vector :default "0, 0, 0") (HitInfo :type Hit%20Result%20Structure%20%28by%20ref%29) (InstigatedBy :type Controller%20Object%20Reference) (DamageCauser :type Actor%20Object%20Reference))
  (Utilities|Struct|SetmembersinDP_RadialDamageData (Variables|Default|GetRadialDamageReplicated) (Utilities|String|ToString(Float) DamageReceived) (Utilities|GetDisplayName DamageType) (Utilities|GetDisplayName InstigatedBy) (Utilities|GetDisplayName DamageCauser) (Utilities|GetDisplayName (Components|GetOwner DamageCauser)) (Utilities|String|ToString(Vector) Origin))
  (Audio|PlaySoundatLocation "/Game/CustomMaps/UGC1908549791/DebugPavlov/Audio/Roblox_Death_Sound_-_OOF__Sound_Effect.Roblox_Death_Sound_-_OOF__Sound_Effect" (.ImpactPoint (Collision|BreakHitResult HitInfo)) "0, 0, 0" 1.0 1.0 0.0 "/Game/CustomMaps/UGC1908549791/DebugPavlov/Audio/Attn_Oof.Attn_Oof" 0 0))

(fn ConstructionScript)

(fn ResetHitData
  (Variables|Default|SetHitDataReplicated (Utilities|Struct|MakeDP_HitData 0 0.0 0.0)))

(fn OnRepHitDataReplicated
  (if (> (.TotalTimesHit (Utilities|Struct|BreakDP_HitData (Variables|Default|GetHitDataReplicated))) 0)
    (Components|Animation|PlayAnimation (Variables|Character|GetMesh) (Utilities|Select :Index (Math|Random|RandomIntegerinRange 0 3) :Option%200 "/Game/CustomMaps/UGC1908549791/PMF/Animations/AnimStarterPack/Hit_React_1.Hit_React_1" :Option%201 "/Game/CustomMaps/UGC1908549791/PMF/Animations/AnimStarterPack/Hit_React_2.Hit_React_2" :Option%202 "/Game/CustomMaps/UGC1908549791/PMF/Animations/AnimStarterPack/Hit_React_3.Hit_React_3" :Option%203 "/Game/CustomMaps/UGC1908549791/PMF/Animations/AnimStarterPack/Hit_React_4.Hit_React_4") false)
    (Audio|PlaySoundatLocation "/Game/CustomMaps/UGC1908549791/DebugPavlov/Audio/Roblox_Death_Sound_-_OOF__Sound_Effect.Roblox_Death_Sound_-_OOF__Sound_Effect" (Transformation|GetActorLocation) "0, 0, 0" 1.0 1.0 0.0 "/Game/CustomMaps/UGC1908549791/DebugPavlov/Audio/Attn_Oof.Attn_Oof" 0 0)))