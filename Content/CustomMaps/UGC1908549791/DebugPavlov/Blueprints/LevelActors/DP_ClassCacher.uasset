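; DP_ClassCacher is a level actor in the DebugPavlov map that can check whether a Pavlov item class resolves from its ID.
; On BeginPlay, after the parent logic, the DebugClasses flag gates a lookup of one hardcoded item enum through GetItemClassByID, logging the found result and class name to the PMF log.
; The graph itself does no caching, and the construction script only calls its parent.
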(event EventBeginPlay
  (bind _returnvalue (Utilities|Enum|LiteralenumEPMF_PavlovItems "NewEnumerator49"))
  (|CallParentFunction)
  (if (Variables|Debug|GetbDebugClasses)
    (bind (_itemclass _bfound) (CallFunction|GetItemClassbyID _returnvalue))
    (CallFunction|AddPMFLog (Utilities|String|Append (Utilities|String|EnumtoString _returnvalue) " Class was found? " (Utilities|String|ToString(Boolean) _bfound) ", Class = " (Utilities|GetClassDisplayName _itemclass)))))

(fn ConstructionScript
  (|CallParentFunction))