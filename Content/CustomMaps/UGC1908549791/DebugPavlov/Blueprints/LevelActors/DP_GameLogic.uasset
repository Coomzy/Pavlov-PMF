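; DP_GameLogic is a game logic Blueprint in the DebugPavlov custom map, apparently a debugging stub.
; Each Tick it calls the parent, then loops over the GameState PlayerArray with an empty loop body.
; Disconnected Append nodes would format the array index, display name and player name, but nothing uses or outputs them.
; The construction script only calls its parent.
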(event EventTick
  (params (DeltaSeconds :type Float%20%28single-precision%29))
  (|CallParentFunction DeltaSeconds)
  (for (_array_element _array_index) (Variables|/Script/Engine.GameStateBase|GetPlayerArray (Game|GetGameState))
    _))

(fn ConstructionScript
  (|CallParentFunction))