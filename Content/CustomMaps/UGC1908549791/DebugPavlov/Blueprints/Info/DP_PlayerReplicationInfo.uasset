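; Per-player replication info for the DebugPavlov map, adding debug actions on top of its PMF parent.
; Become Character and Ghost pass the pawn's transform to Server events that respawn the player there via PMF game logic; Clone chains Ghost then Character.
; It also resets hit data on all damage characters, logs leaves and rejoins on authority, and increments and saves a load counter when game info loads.
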(event Custom|BecomeClone
  (CallFunction|BecomeGhost)
  (Utilities|FlowControl|Delay 0.2)
  (CallFunction|BecomeCharacter))

(event Custom|ServerResetHitData
  (bind _outactors (Actor|GetAllActorsOfClass "/Game/CustomMaps/UGC1908549791/DebugPavlov/Blueprints/LevelActors/DP_DamageCharacter.DP_DamageCharacter_C"))
  (for _array_element _outactors
    (Default|ResetHitData _array_element)))

(event Custom|ServerBecomeGhost
  (params (Loc :type Vector) (Rot :type Rotator))
  (Default|RespawnPlayer (CallFunction|GetPMFGameLogic) self true true (Math|Transform|MakeTransform Loc Rot))
  (Utilities|FlowControl|Delay 0.2)
  (Default|InitSpawnedPlayer (CallFunction|GetPMFGameLogic) self))

(event Custom|ServerBecomeCharacter
  (params (Loc :type Vector) (Rot :type Rotator))
  (Default|RespawnPlayer (CallFunction|GetPMFGameLogic) self false true (Math|Transform|MakeTransform Loc Rot))
  (Utilities|FlowControl|Delay 0.2)
  (Default|InitSpawnedPlayer (CallFunction|GetPMFGameLogic) self))

(event Custom|BecomeGhost
  (bind _pawn (CallFunction|GetPlayerPawn))
  (CallFunction|ServerBecomeGhost (Transformation|GetActorLocation _pawn) (Transformation|GetActorRotation _pawn)))

(event Custom|BecomeCharacter
  (bind _pawn (CallFunction|GetPlayerPawn))
  (CallFunction|ServerBecomeCharacter (Transformation|GetActorLocation _pawn) (Transformation|GetActorRotation _pawn)))

(event EventBeginPlay
  (|CallParentFunction)
  (Networking|SwitchHasAuthority))

(event EventPlayerLeftServer
  (|CallParentFunction)
  (Networking|SwitchHasAuthority
    (:Authority
      (CallFunction|AddPMFLog (Utilities|String|Append (CallFunction|GetPlayerName) " left the server :'(")))))

(event EventPlayerRejoinServer
  (params (NewPlayerState :type Player%20State%20Object%20Reference))
  (|CallParentFunction NewPlayerState)
  (Networking|SwitchHasAuthority
    (:Authority
      (CallFunction|AddPMFLog (Utilities|String|Append (CallFunction|GetPlayerName) " re-joined the server!!!")))))

(fn ConstructionScript
  (|CallParentFunction))

(fn LoadGameInfo
  (bind _outsavedata (|CallParentFunction))
  (bind _asdp_save_game (Utilities|Casting|CastToDP_SaveGame _outsavedata)
    (:then
      (Math|Integer|IncrementInt (Variables|/Game/CustomMaps/UGC1908549791/DebugPavlov/Blueprints/Data/Saving/DP_SaveGame.DP_SaveGame_C|GetTimesLoaded _asdp_save_game)
        (:%20%20
          (CallFunction|SaveGameInfo)
          (return _asdp_save_game))))
    (:CastFailed
      (return _outsavedata))))