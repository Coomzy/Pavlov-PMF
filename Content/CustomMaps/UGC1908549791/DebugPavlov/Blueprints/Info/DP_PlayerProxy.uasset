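; Player proxy for the DebugPavlov custom map that adds debug controller shortcuts for jumping and cloning.
; Pressing either trigger calls JumpPlayer if that hand holds no item, using the player's handedness to pick the hand to check.
; Holding Scoreboard and CycleFireMode together, from either controller, calls BecomeClone on the DP_PlayerReplicationInfo.
; Left and right buttons share one held flag per action, so releasing either side clears it.
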(event Custom|AttemptClone
  (if (and (Variables|Default|GetbScoreboardIsDown) (Variables|Default|GetbCycleFireModeIsDown))
    (bind _asdp_player_replication_info (Utilities|Casting|CastToDP_PlayerReplicationInfo (.OwningPRI (CallFunction|GetOwningPRI))))
    (Default|BecomeClone _asdp_player_replication_info)))

(event Input|ActionEvents|InputActionScoreboardLeft
  (params (Key :type Key%20Structure))
  (:Pressed
    (Variables|Default|SetbScoreboardIsDown true)
    (CallFunction|AttemptClone))
  (:Released
    (Variables|Default|SetbScoreboardIsDown false)))

(event Input|ActionEvents|InputActionTriggerLeft
  (params (Key :type Key%20Structure))
  (:Pressed
    (bind _bhasitem (Class|PavlovPlayerProxy|GetHeldItem (not (Default|IsRightHanded (.OwningPRI (CallFunction|GetOwningPRI))))))
    (if (not _bhasitem)
      (CallFunction|JumpPlayer))))

(event Input|ActionEvents|InputActionTriggerRight
  (params (Key :type Key%20Structure))
  (:Pressed
    (bind _bhasitem (Class|PavlovPlayerProxy|GetHeldItem (Default|IsRightHanded (.OwningPRI (CallFunction|GetOwningPRI)))))
    (if (not _bhasitem)
      (CallFunction|JumpPlayer))))

(event Input|ActionEvents|InputActionScoreboardRight
  (params (Key :type Key%20Structure))
  (:Pressed
    (Variables|Default|SetbScoreboardIsDown true)
    (CallFunction|AttemptClone))
  (:Released
    (Variables|Default|SetbScoreboardIsDown false)))

(event Input|ActionEvents|InputActionCycleFireModeLeft
  (params (Key :type Key%20Structure))
  (:Pressed
    (Variables|Default|SetbCycleFireModeIsDown true)
    (CallFunction|AttemptClone))
  (:Released
    (Variables|Default|SetbCycleFireModeIsDown false)))

(event Input|ActionEvents|InputActionCycleFireModeRight
  (params (Key :type Key%20Structure))
  (:Pressed
    (Variables|Default|SetbCycleFireModeIsDown true)
    (CallFunction|AttemptClone))
  (:Released
    (Variables|Default|SetbCycleFireModeIsDown false)))

(fn ConstructionScript
  (|CallParentFunction))