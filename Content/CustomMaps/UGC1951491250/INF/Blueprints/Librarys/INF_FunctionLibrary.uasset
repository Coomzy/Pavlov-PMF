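; INF_FunctionLibrary is a Blueprint function library that gives access to the INF map's globals, game logic and sound manager.
; The game logic and sound manager getters cast the PMF framework's accessors to their INF subclasses.
; Only the sound manager getter reports validity.
; The globals getter constructs a new INF_GlobalVariables object on every call rather than returning a shared instance.
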(fn GetINFGlobals
  (bind _returnvalue (Game|ConstructObjectfromClass "/Game/CustomMaps/UGC1951491250/INF/Blueprints/Objects/INF_GlobalVariables.INF_GlobalVariables_C" (LocalVariables|Get__WorldContext)))
  (return _returnvalue))

(fn GetINFGameLogic
  (bind _asinf_game_logic (Utilities|Casting|CastToINF_GameLogic (CallFunction|GetPMFGameLogic (LocalVariables|Get__WorldContext)))
    (:then
      (return _asinf_game_logic))
    (:CastFailed
      (return 0))))

(fn GetINFSoundManager
  (bind _asinf_sound_manager (Utilities|Casting|CastToINF_SoundManager (.PMFSoundManager (CallFunction|GetPMFSoundManager (LocalVariables|Get__WorldContext))))
    (:then
      (return _asinf_sound_manager true))
    (:CastFailed
      (return 0 false))))