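; Player replication info for the Infection game mode, tracking zombie and alpha-zombie status and handling that player's abilities and announcements.
; Spawning as a zombie attaches an energy sword, which is cleaned up on death or leaving.
; Locally controlled launches drive configurable jumps and airborne zombie sword lunges, the latter with a server-time cooldown and multicast sound.
; It also spawns the last-man-standing actor and queues killing-spree and multi-kill award sounds.
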(event Custom|MulticastLungeSound
  (bind _returnvalue (Math|Random|RandomIntegerinRange 0 2))
  (bind _pawn (CallFunction|GetPlayerPawn))
  (bind _curenergysword (Variables|DataReplicated|GetCurEnergySword))
  (bind _returnvalue_2 (Utilities|Select :Index _returnvalue :Option%200 "/Game/CustomMaps/UGC1951491250/INF/Audio/EnergySword/Lunge/energy_sword_lunge_hum1.energy_sword_lunge_hum1" :Option%201 "/Game/CustomMaps/UGC1951491250/INF/Audio/EnergySword/Lunge/energy_sword_lunge_hum2.energy_sword_lunge_hum2" :Option%202 "/Game/CustomMaps/UGC1951491250/INF/Audio/EnergySword/Lunge/energy_sword_lunge_hum3.energy_sword_lunge_hum3"))
  (if (not (or (CallFunction|IsLocalPRI) (Networking|IsDedicatedServer))) ; Remote Player
    (Utilities|IsValid _curenergysword
      (:Is%20Valid
        (Audio|PlaySoundatLocation _returnvalue_2 (Transformation|GetActorLocation _curenergysword) "0, 0, 0" 1.0 1.0 0.0 0 0 0))
      (:Is%20Not%20Valid
        (Utilities|IsValid _pawn
          (:Is%20Valid
            (Audio|PlaySoundatLocation _returnvalue_2 (Transformation|GetActorLocation _pawn) "0, 0, 0" 1.0 1.0 0.0 0 0 0)))))))

(event EventPlayerDied
  (|CallParentFunction)
  (Utilities|IsValid (Variables|DataReplicated|GetCurEnergySword)
    (:Is%20Valid
      (Default|OwnerDied (Variables|DataReplicated|GetCurEnergySword))
      (Variables|DataReplicated|SetCurEnergySword 0))))

(event EventPlayerSpawned
  (|CallParentFunction)
  (if (.bIsZombie (CallFunction|IsZombie))
    (CallFunction|SpawnEnergySword)))

(event EventAddKills
  (Variables|Data|SetCachedLastKillTime (Variables|Default|GetLastKillTime))
  (|CallParentFunction)
  (if (Variables|/Game/CustomMaps/UGC1951491250/INF/Blueprints/LevelActors/Core/INF_GameLogic.INF_GameLogic_C|GetbUseGameAwardSystem (CallFunction|GetINFGameLogic))
    (CallFunction|CheckKillingSpree)
    (CallFunction|CheckMultiKill (Variables|Data|GetCachedLastKillTime))))

(event EventClientInitialization
  (|CallParentFunction)
  (if (CallFunction|IsLocalPRI)
    (Default|PlayInfectionAnnouncement (.AsINF%20Sound%20Manager (CallFunction|GetINFSoundManager)))))

(event EventPlayerLeftServer
  (|CallParentFunction)
  (Utilities|IsValid (Variables|DataReplicated|GetCurEnergySword)
    (:Is%20Valid
      (Actor|DestroyActor (Variables|DataReplicated|GetCurEnergySword)))))

(fn ConstructionScript
  (|CallParentFunction))

(fn IsZombie
  (return (== (CallFunction|GetTeamIndex) (Variables|/Game/CustomMaps/UGC1951491250/INF/Blueprints/Objects/INF_GlobalVariables.INF_GlobalVariables_C|GetTeamZombieIndex (CallFunction|GetINFGlobals))) (Variables|DataReplicated|GetbIsAlphaZombie)))

(fn JumpPlayer
  (bind _bcanjump (CallFunction|CanJump))
  (if _bcanjump
    (bind _ascharacter (Utilities|Casting|CastToCharacter (Variables|/Script/Engine.PlayerState|GetPawnPrivate (CallFunction|GetOwningPlayerState))))
    (if (not (AI|Components|NavMovement|IsFalling (Variables|/Script/Engine.Character|GetCharacterMovement _ascharacter)))
      (if (Pawn|IsLocallyControlled _ascharacter)
        (Character|LaunchCharacter _ascharacter (Math|Vector|MakeVector 0.0 0.0 (Variables|Config-INF|GetJumpForce)) false true)))))

(fn CanJump
  (if (Variables|Config-INF|GetbAllowJumping)
    (if (Variables|Config-INF|GetbOnlyAllowZombiesJumping)
      (return (.bIsZombie (CallFunction|IsZombie)))
      (else
        (return true)))
    (else
      (return false))))

(fn SpawnEnergySword
  (bind _returnvalue (Game|SpawnActorfromClass (Variables|Config-INF|GetEnergySwordClass) (Math|Transform|MakeTransform "0, 0, 0") "AlwaysSpawn" (CallFunction|GetPlayerController) self (.Pawn (CallFunction|GetPlayerPawn))))
  (bind _output_get (Variables|DataReplicated|SetCurEnergySword _returnvalue))
  (Transformation|AttachActorToActor _output_get (Components|GetOwner (CallFunction|GetController true)) "None" "SnapToTarget" "SnapToTarget" "KeepRelative" true))

(fn BecomeAlphaZombie
  (Variables|DataReplicated|SetbIsAlphaZombie true)
  (Default|PlayInfectedAnnouncement (.AsINF%20Sound%20Manager (CallFunction|GetINFSoundManager)) self))

(fn BecomeHuman
  (Variables|DataReplicated|SetbIsAlphaZombie false))

(fn LungePlayer
  (bind (_character _bisvalid) (CallFunction|GetPlayerCharacter))
  (bind _curenergysword (Variables|DataReplicated|GetCurEnergySword))
  (bind (_returnvalue _bisusingtarget _target) (Default|GetSwordLungeDir _curenergysword))
  (bind _bcanlunge (CallFunction|CanLunge))
  (if _bcanlunge
    (if _bisvalid
      (if (Pawn|IsLocallyControlled _character)
        (Utilities|IsValid _curenergysword
          (:Is%20Valid
            (bind _modlungedir (CallFunction|ModifyLungeDir (Math|Vector|Normalize _returnvalue) _bisusingtarget _target))
            (Character|LaunchCharacter _character _modlungedir (Variables|Config-INF|GetbLungeOverridesVelocityXY) (Variables|Config-INF|GetbLungeOverridesVelocityZ))
            (Variables|Data|SetLastLungeTime (GameState|GetServerWorldTimeSeconds (Game|GetGameState)))
            (Audio|PlaySound2D (Utilities|Select :Index (Math|Random|RandomIntegerinRange 0 2) :Option%200 "/Game/CustomMaps/UGC1951491250/INF/Audio/EnergySword/Lunge/energy_sword_lunge_hum1.energy_sword_lunge_hum1" :Option%201 "/Game/CustomMaps/UGC1951491250/INF/Audio/EnergySword/Lunge/energy_sword_lunge_hum2.energy_sword_lunge_hum2" :Option%202 "/Game/CustomMaps/UGC1951491250/INF/Audio/EnergySword/Lunge/energy_sword_lunge_hum3.energy_sword_lunge_hum3") 1.0 1.0 0.0 0 0)
            (CallFunction|MulticastLungeSound)))))))

(fn CanLunge
  (if (.bIsZombie (CallFunction|IsZombie))
    (if (.IsFalling (CallFunction|IsCharacterFalling)) ; Lunge on Ground is hard, just removed it for now\nMight try and add it later
      (Utilities|IsValid (Variables|DataReplicated|GetCurEnergySword)
        (:Is%20Valid
          (return (>= (- (GameState|GetServerWorldTimeSeconds (Game|GetGameState)) (Variables|Data|GetLastLungeTime)) (Variables|Config-INF|GetLungeCooldownTime))))
        (:Is%20Not%20Valid
          (return false)))
      (else
        (return false)))
    (else
      (return false))))

(fn ResetLungeCooldown
  (Variables|Data|SetLastLungeTime (.LastLungeTime (Utilities|GetClassDefaults "INF_PlayerReplicationInfo_C"))))

(fn ModifyLungeDir
  (params (LungeDir :type Vector) (bIsUsingTarget :type Boolean) (Target :type Actor%20Object%20Reference))
  (bind (_character _bisvalid) (CallFunction|GetPlayerCharacter))
  (bind (_x _y) (Math|Vector|BreakVector LungeDir))
  (bind _returnvalue (Math|Vector|MakeVector _x _y 0.0))
  (bind _returnvalue_2 (Math|Vector|Normalize _returnvalue))
  (bind (_x_2 _y_2) (Math|Vector|BreakVector _returnvalue_2))
  (if _bisvalid
    (if (not (AI|Components|NavMovement|IsFalling (Variables|/Script/Engine.Character|GetCharacterMovement _character))) ; Are We Grounded?
      (if (> (Math|Vector|DotProduct (Math|Vector|MakeVector 0.0 0.0 1.0) (Math|Vector|Normalize LungeDir)) 0.1) ; Aiming At/Near Ground
        (return (* (Math|Vector|Normalize (Math|Vector|MakeVector _x_2 _y_2 0.1)) (Variables|Config-INF|GetLungeForce)))
        (else
          (return (* (Math|Vector|Normalize LungeDir) (Variables|Config-INF|GetLungeForce)))))
      (else
        (LocalVariables|SetCachedZ (.Z (Math|Vector|BreakVector (Math|Vector|Normalize LungeDir))))
        (return (* (Math|Vector|Normalize LungeDir) (Variables|Config-INF|GetLungeForce))) ; Temp To Test Normal Lunging
      ))
    (else
      (return LungeDir))))

(fn ApplyLastManStanding
  (Game|SpawnActorfromClass (Variables|/Game/CustomMaps/UGC1951491250/INF/Blueprints/LevelActors/Core/INF_GameLogic.INF_GameLogic_C|GetLastManStandingActorClass (CallFunction|GetINFGameLogic)) (Math|Transform|MakeTransform "0, 0, 0") "AlwaysSpawn" (CallFunction|GetPlayerController) self 0))

(fn CheckKillingSpree
  (if (not (not (CallFunction|IsDead)))
    (if (Utilities|Map|Contains (Variables|Config-INF|GetKillingSpreeAwards) (Variables|Default|GetKillsThisLife))
      (Default|PlayQueuedSoundforPRI (.PMFSoundManager (CallFunction|GetPMFSoundManager)) self (.Value (Utilities|Map|Find (Variables|Config-INF|GetKillingSpreeAwards) (Variables|Default|GetKillsThisLife))) true))))

(fn CheckMultiKill
  (params (ActualLastKillTime :type Float%20%28single-precision%29))
  (if (<= (- (GameState|GetServerWorldTimeSeconds (Game|GetGameState)) ActualLastKillTime) (Variables|Config-INF|GetMultiKillTimeGap))
    (Math|Integer|IncrementInt (Variables|Data|GetMultiKillCount)
      (:%20%20
        (if (Utilities|Map|Contains (Variables|Config-INF|GetMultiKillAwards) (Variables|Data|GetMultiKillCount))
          (Default|PlayQueuedSoundforPRI (.PMFSoundManager (CallFunction|GetPMFSoundManager)) self (.Value (Utilities|Map|Find (Variables|Config-INF|GetMultiKillAwards) (Variables|Data|GetMultiKillCount))) true))))
    (else
      (Variables|Data|SetMultiKillCount 1))))