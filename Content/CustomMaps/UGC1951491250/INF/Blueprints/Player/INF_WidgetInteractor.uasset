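; INF_WidgetInteractor is the player widget interactor for the INF mode, deciding when UI interaction is enabled.
; It overrides IsInteractionSystemOn, returning false unless the required-role check passes.
; For zombie players, interaction is on only while their spawned scoreboard is open.
; Non-zombies, and owners without an INF_PlayerReplicationInfo, defer to the parent implementation.
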(fn ConstructionScript
  (|CallParentFunction))

(fn IsInteractionSystemon
  (if (CallFunction|IsRequiredRole)
    (bind _asinf_player_replication_info (Utilities|Casting|CastToINF_PlayerReplicationInfo (Variables|Default|GetOwningPRI))
      (:then
        (if (not (.bIsZombie (Default|IsZombie _asinf_player_replication_info)))
          (bind _bison (|CallParentFunction))
          (return _bison)
          (else
            (return (Variables|/Game/CustomMaps/UGC1951491250/PMF/Blueprints/Player/PMF_CustomScoreboard.PMF_CustomScoreboard_C|GetbScoreboardIsOpen (Variables|/Game/CustomMaps/UGC1951491250/PMF/Blueprints/Info/PMF_PlayerReplicationInfo.PMF_PlayerReplicationInfo_C|GetSpawnedScoreboard (Variables|Default|GetOwningPRI)))))))
      (:CastFailed
        (bind _bison_2 (|CallParentFunction))
        (return _bison_2)))
    (else
      (return false))))