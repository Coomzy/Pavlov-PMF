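; INF_PlayerInput is the player input Blueprint for the INF custom map, turning trigger presses on the VR controllers into lunge and jump moves.
; It extends the parent trigger handler, then casts the owning PRI to INF_PlayerReplicationInfo, which performs the move.
; A right-controller press lunges only for right-handed players; every other press jumps, so left-handed players never lunge from this handler.
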(event EventInputTriggerButton
  (params (bIsRightController :type Boolean) (bIsButtonDown :type Boolean))
  (|CallParentFunction bIsRightController bIsButtonDown)
  (if bIsButtonDown
    (bind _asinf_player_replication_info (Utilities|Casting|CastToINF_PlayerReplicationInfo (Variables|Default|GetOwningPRI)))
    (if (and bIsRightController (CallFunction|IsRightHanded)) ; Is Dominant Hand
      (Default|LungePlayer _asinf_player_replication_info)
      (else
        (Default|JumpPlayer _asinf_player_replication_info)))))

(fn ConstructionScript
  (|CallParentFunction))