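; PMF_TeamReplicationInfo is a Blueprint in the PMF custom map content that represents one team and tracks the players on it.
; Join and leave functions maintain the TeamPRIs list of player replication infos, and joining also stamps the team's index onto the player's PRI.
; Helpers report player count and whether the team has members, and allow respawn for any team except the spectator team defined in PMF globals.
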(fn ConstructionScript)

(fn PlayerJoinTeam
  (params (PRI :type PMF%20Player%20Replication%20Info%20Object%20Reference))
  (Utilities|Array|AddUnique (Variables|DataReplicated|GetTeamPRIs) PRI)
  (Variables|/Game/CustomMaps/UGC1951491250/PMF/Blueprints/Info/PMF_PlayerReplicationInfo.PMF_PlayerReplicationInfo_C|SetTeamIndex PRI (Variables|DataReplicated|GetTeamIndex)))

(fn PlayerLeaveTeam
  (params (PRI :type PMF%20Player%20Replication%20Info%20Object%20Reference))
  (Utilities|Array|RemoveItem (Variables|DataReplicated|GetTeamPRIs) PRI))

(fn GetPlayerCount
  (return (Utilities|Array|Length (Variables|DataReplicated|GetTeamPRIs))))

(fn CanPlayerRespawn
  (params (PRI :type PMF%20Player%20Replication%20Info%20Object%20Reference))
  (return (!= (Variables|DataReplicated|GetTeamIndex) (Variables|/Game/CustomMaps/UGC1951491250/PMF/Blueprints/Objects/PMF_GlobalVariables.PMF_GlobalVariables_C|GetTeamSpectatorIndex (CallFunction|GetPMFGlobals)))))

(fn HasAnyPlayers
  (return (> (CallFunction|GetPlayerCount) 0)))