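; PMF character proxy info that manages the lifetime of a player info actor tied to an owning PRI.
; On BeginPlay it spawns the configured player info class at the world origin, if the PMF game logic enables it and none exists yet.
; PlayerDied sets the dead flag, whose RepNotify destroys the spawned info actor.
; PlayerLeftServer is an empty stub.
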(event EventBeginPlay
  (|CallParentFunction)
  (Creation|SpawnPlayerInfo))

(fn ConstructionScript
  (|CallParentFunction))

(fn SpawnPlayerInfo
  (if (Variables|/Game/CustomMaps/UGC1951491250/PMF/Blueprints/LevelActors/CORE/PMF_GameLogic.PMF_GameLogic_C|GetbUsePMFPlayerInfo (CallFunction|GetPMFGameLogic))
    (Utilities|IsValid (Variables|Data|GetSpawnedPlayerInfo)
      (:Is%20Not%20Valid
        (bind _returnvalue (Game|SpawnActorfromClass (Variables|Default|GetPlayerInfoClass) (Math|Transform|MakeTransform "0, 0, 0") "AlwaysSpawn" 0 (Variables|DataReplicated|GetOwningPRI) 0))
        (Variables|Data|SetSpawnedPlayerInfo _returnvalue)))))

(fn OnRepBIsDead
  (Creation|DestroyPlayerInfo))

(fn DestroyPlayerInfo
  (Utilities|IsValid (Variables|Data|GetSpawnedPlayerInfo)
    (:Is%20Valid
      (Actor|DestroyActor (Variables|Data|GetSpawnedPlayerInfo)))))

(fn PlayerDied
  (Variables|DataReplicated|SetbIsDead true))

(fn PlayerLeftServer)