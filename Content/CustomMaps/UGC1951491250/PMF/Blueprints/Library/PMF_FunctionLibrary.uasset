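; Static helper library for the PMF Pavlov mod framework, giving global access to its subsystems and shared utilities.
; Most accessors route through PMF_Singleton, cached as the GameState's Owner, to reach game logic, class cacher, sound manager and debug handler.
; Constant-holder objects are constructed on demand for globals and Pavlov indices and class names.
; Also provides build-gated logging, random item rolls, asset lookup, vector math and Pavlov character and game-over screen tweaks.
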(fn SetPMFGameLogicbyRef
  (params (PMFGameLogicByRef :type PMF%20Game%20Logic%20Object%20Reference%20%28by%20ref%29))
  (bind ___worldcontext (LocalVariables|Get__WorldContext))
  (bind _pmfgamelogic (Getters|GetPMFGameLogic ___worldcontext))
  (Utilities|IsValid _pmfgamelogic
    (:Is%20Valid
      (|SetBy-RefVar PMFGameLogicByRef _pmfgamelogic))))

(fn GetPMFGameLogic
  (bind ___worldcontext (LocalVariables|Get__WorldContext))
  (bind _pmfsingleton (Getters|GetPMFSingleton ___worldcontext))
  (Utilities|IsValid _pmfsingleton
    (:Is%20Valid
      (return (Default|GetPMFGameLogic _pmfsingleton)))
    (:Is%20Not%20Valid
      (return 0))))

(fn RandomItemtoType
  (params (RandomType :type EPMF_ItemID%20Enum :default "NewEnumerator42"))
  (bind ___worldcontext (LocalVariables|Get__WorldContext))
  (if (Utilities|Enum|Equal(Enum) RandomType "NewEnumerator43")
    (bind _randomindex (Items|GetRandomIndexBetween "NewEnumerator0" "NewEnumerator41" (LocalVariables|Get__WorldContext)))
    (return _randomindex)
    (elif (Utilities|Enum|Equal(Enum) RandomType "NewEnumerator44")
      (bind _randomindex_2 (Items|GetRandomIndexBetween "NewEnumerator0" "NewEnumerator26" ___worldcontext))
      (return _randomindex_2)
      (elif (Utilities|Enum|Equal(Enum) RandomType "NewEnumerator45")
        (bind _randomindex_3 (Items|GetRandomIndexBetween "NewEnumerator27" "NewEnumerator30" ___worldcontext))
        (return _randomindex_3)
        (elif (Utilities|Enum|Equal(Enum) RandomType "NewEnumerator46")
          (bind _randomindex_4 (Items|GetRandomIndexBetween "NewEnumerator32" "NewEnumerator39" (LocalVariables|Get__WorldContext)))
          (return _randomindex_4)
          (else
            (return RandomType)))))))

(fn GetRandomIndexBetween
  (params (FirstIndex :type EPMF_ItemID%20Enum :default "NewEnumerator0") (LastIndex :type EPMF_ItemID%20Enum :default "NewEnumerator41"))
  (return (Utilities|Enum|ByteToEnumEPMF_ItemID (Math|Conversions|ToByte(Integer) (Math|Random|RandomIntegerinRange (Math|Conversions|ToInteger(Byte) FirstIndex) (Math|Conversions|ToInteger(Byte) LastIndex))))))

(fn IsItemTypeRandom
  (params (ItemType :type EPMF_ItemID%20Enum :default "NewEnumerator42"))
  (return (>= ItemType (Utilities|Enum|ByteToEnumEPMF_ItemID (Utilities|Enum|LiteralenumEPMF_ItemID "NewEnumerator43")))))

(fn CheckItembyName
  (params (CheckingActorName :type String) (CheckingActor :type Actor%20Object%20Reference))
  (if (or (Utilities|IsValid (Actor|GetComponentbyClass CheckingActor "/Script/Engine.SkeletalMeshComponent")) (Utilities|IsValid (Actor|GetComponentbyClass CheckingActor "/Script/Engine.StaticMeshComponent"))) ; Items Have To Have Skeletal Or Static Mesh Components?
    (if (Utilities|Enum|Equal(Enum) CheckingActorName (Utilities|GetClassDisplayName (Utilities|GetClass CheckingActor))) ; Item Found?
      (return true)
      (else
        (return false)))
    (else
      (return false))))

(fn GetPMFSingleton
  (bind ___worldcontext (LocalVariables|Get__WorldContext))
  (bind _returnvalue (Game|GetGameState ___worldcontext))
  (Utilities|IsValid _returnvalue
    (:Is%20Valid
      (bind _aspmf_singleton (Utilities|Casting|CastToPMF_Singleton (Components|GetOwner _returnvalue))
        (:then
          (return _aspmf_singleton))
        (:CastFailed
          (bind _outactors (Actor|GetAllActorsOfClass (LocalVariables|Get__WorldContext) "/Game/CustomMaps/UGC1951491250/PMF/Blueprints/LevelActors/CORE/PMF_Singleton.PMF_Singleton_C"))
          (Actor|SetOwner (Game|GetGameState (LocalVariables|Get__WorldContext)) (Utilities|Array|Get(acopy) _outactors))
          (return (Utilities|Array|Get(acopy) _outactors)))))
    (:Is%20Not%20Valid
      (return 0) ; No Game State = Fucked Or In Editor
    )))

(fn GetLocalPRI
  (bind _localpri (Default|GetLocalPRI (Getters|GetPMFGameLogic (LocalVariables|Get__WorldContext))))
  (return _localpri))

(fn AddPMFLog
  (params (LogText :type String))
  (Default|AddLog (Default|GetPMFDebugHandler (Getters|GetPMFSingleton (LocalVariables|Get__WorldContext))) LogText))

(fn AddPMFConstantLog
  (params (LogName :type String) (LogText :type String))
  (Default|AddConstantLog (Default|GetPMFDebugHandler (Getters|GetPMFSingleton (LocalVariables|Get__WorldContext))) LogName LogText))

(fn GetPavlovAssetbyPath
  (params (Path :type Name) (AssetName :type Name) (bLogAsset :type Boolean))
  (for (_array_element _array_index) (.OutAssetData (Class|AssetRegistry|GetAssetsbyPath (Class|AssetRegistryHelpers|GetAssetRegistry) Path false false))
    (if (Utilities|Name|Equal(Name) (.AssetName (Utilities|Struct|BreakAssetData _array_element)) AssetName)
      (if (Utilities|Name|Equal(Name) (.AssetClass (Utilities|Struct|BreakAssetData _array_element)) "Blueprint")
        (Logging|AddPMFLogBeta "WARNING GetPavlovAssetByPath() does NOT work with blueprint classes" (LocalVariables|Get__WorldContext)))
      (if bLogAsset
        (Logging|AddPMFLogBeta (Utilities|String|Append "[" (Utilities|String|ToString(Integer) _array_index) "] 
" (Utilities|String|ToString(Name) (.ObjectPath (Utilities|Struct|BreakAssetData _array_element))) " 
" (Utilities|String|ToString(Name) (.PackageName (Utilities|Struct|BreakAssetData _array_element))) " 
" (Utilities|String|ToString(Name) (.PackagePath (Utilities|Struct|BreakAssetData _array_element))) " 
" (Utilities|String|ToString(Name) (.AssetName (Utilities|Struct|BreakAssetData _array_element))) " 
" (Utilities|String|ToString(Name) (.AssetClass (Utilities|Struct|BreakAssetData _array_element)))) (LocalVariables|Get__WorldContext)))
      (return _array_element true)))
  (return "" false))

(fn GetItemClassbyID
  (params (ItemID :type EPMF_ItemID%20Enum :default "NewEnumerator42"))
  (bind (_itemclass _bfound) (Default|GetItemClassbyID (Default|GetPMFClassCacher (Getters|GetPMFSingleton (LocalVariables|Get__WorldContext))) ItemID))
  (return _itemclass _bfound))

(fn GetPMFClassCacher
  (bind ___worldcontext (LocalVariables|Get__WorldContext))
  (bind _pmfsingleton (Getters|GetPMFSingleton ___worldcontext))
  (Utilities|IsValid _pmfsingleton
    (:Is%20Valid
      (return (Default|GetPMFClassCacher _pmfsingleton)))
    (:Is%20Not%20Valid
      (return 0))))

(fn AddVelocitytoCharacter
  (params (Character :type Character%20Object%20Reference) (Force :type Vector))
  (bind _charactermovement (Variables|/Script/Engine.Character|GetCharacterMovement Character))
  (Utilities|IsValid Character
    (:Is%20Valid
      (Variables|/Script/Engine.MovementComponent|SetVelocity _charactermovement (+ Force (Variables|/Script/Engine.MovementComponent|GetVelocity _charactermovement))))))

(fn GetPMFGlobals
  (bind _returnvalue (Game|ConstructObjectfromClass "/Game/CustomMaps/UGC1951491250/PMF/Blueprints/Objects/PMF_GlobalVariables.PMF_GlobalVariables_C" (LocalVariables|Get__WorldContext)))
  (return _returnvalue))

(fn GetItemIDbyClass
  (params (ItemClass :type Actor%20Class%20Reference))
  (bind _itemid (Default|GetItemIDbyClass (Default|GetPMFClassCacher (Getters|GetPMFSingleton (LocalVariables|Get__WorldContext))) ItemClass))
  (return _itemid))

(fn GetPMFSoundManager
  (bind ___worldcontext (LocalVariables|Get__WorldContext))
  (bind _pmfsingleton (Getters|GetPMFSingleton ___worldcontext))
  (bind _pmfsoundmanager (Default|GetPMFSoundManager _pmfsingleton))
  (return _pmfsoundmanager (Utilities|IsValid _pmfsoundmanager)))

(fn GetBuildType
  (return (Variables|/Game/CustomMaps/UGC1951491250/PMF/Blueprints/LevelActors/CORE/PMF_GameLogic.PMF_GameLogic_C|GetPMFBuildType (Getters|GetPMFGameLogic (LocalVariables|Get__WorldContext)))))

(fn IsDevelopmentBuild
  (return (Utilities|Enum|Equal(Enum) (BuildInfo|GetBuildType (LocalVariables|Get__WorldContext)) "NewEnumerator0")))

(fn IsBetaBuild
  (return (Utilities|Enum|Equal(Enum) (BuildInfo|GetBuildType (LocalVariables|Get__WorldContext)) "NewEnumerator1")))

(fn IsLiveBuild
  (return (Utilities|Enum|Equal(Enum) (BuildInfo|GetBuildType (LocalVariables|Get__WorldContext)) "NewEnumerator2")))

(fn AddPMFLogDevelopment
  (params (LogText :type String))
  (if (BuildInfo|IsDevelopmentBuild (LocalVariables|Get__WorldContext))
    (Logging|AddPMFLog LogText (LocalVariables|Get__WorldContext))))

(fn AddPMFLogBeta
  (params (LogText :type String))
  (if (not (BuildInfo|IsLiveBuild (LocalVariables|Get__WorldContext)))
    (Logging|AddPMFLog LogText (LocalVariables|Get__WorldContext))))

(fn GetPMFVersion
  (return (Variables|/Game/CustomMaps/UGC1951491250/PMF/Blueprints/Objects/PMF_GlobalVariables.PMF_GlobalVariables_C|GetPMFVersion (Globals|GetPMFGlobals (LocalVariables|Get__WorldContext)))))

(fn GetBuildVersion
  (return (Variables|/Game/CustomMaps/UGC1951491250/PMF/Blueprints/LevelActors/CORE/PMF_GameLogic.PMF_GameLogic_C|GetPMFBuildVersion (Getters|GetPMFGameLogic (LocalVariables|Get__WorldContext)))))

(fn IsMControllerHoldingItem
  (params (MC :type Motion%20Controller%20Component%20Object%20Reference) (ItemClass :type Actor%20Class%20Reference))
  (Utilities|IsValid MC
    (:Is%20Valid
      (if (!= ItemClass 0)
        (for _array_element (Actor|GetAttachedActors (Components|GetOwner MC))
          (if (== (Utilities|GetClass _array_element) ItemClass)
            (return _array_element true true)))
        (return 0 false true)
        (else
          (return 0 false false))))
    (:Is%20Not%20Valid
      (return 0 false false))))

(fn GetLocalPMFCheatManager
  (return (Default|GetPMFCheatManager (Getters|GetLocalPRI (LocalVariables|Get__WorldContext)))))

(fn GetPavlovIndexs
  (bind _returnvalue (Game|ConstructObjectfromClass "/Game/CustomMaps/UGC1951491250/PMF/Blueprints/Objects/PMF_PavlovIndexs.PMF_PavlovIndexs_C" (LocalVariables|Get__WorldContext)))
  (return _returnvalue))

(fn ApplyMaterialtoCharacter
  (params (Character :type Character%20Object%20Reference) (MaterialToApply :type Material%20Interface%20Object%20Reference) (bBodyOnly :type Boolean) (bHelmetOnly :type Boolean))
  (bind ___worldcontext (LocalVariables|Get__WorldContext))
  (bind ___worldcontext_2 (LocalVariables|Get__WorldContext))
  (bind _indexs (Globals|GetPavlovIndexs ___worldcontext_2))
  (bind _indexs_2 (Globals|GetPavlovIndexs ___worldcontext))
  (if (not (Networking|IsDedicatedServer (LocalVariables|Get__WorldContext))) ; Waste Of Effort
    (Utilities|IsValid Character
      (:Is%20Valid
        (Utilities|IsValid MaterialToApply
          (:Is%20Valid
            (for _index (range (select (and bHelmetOnly (not bBodyOnly)) (Variables|/Game/CustomMaps/UGC1951491250/PMF/Blueprints/Objects/PMF_PavlovIndexs.PMF_PavlovIndexs_C|GetInventoryCharacterHelmetMeshOffset _indexs_2) (Variables|/Game/CustomMaps/UGC1951491250/PMF/Blueprints/Objects/PMF_PavlovIndexs.PMF_PavlovIndexs_C|GetInventoryCharacterBodyMeshOffset _indexs_2)) (select (and bBodyOnly (not bHelmetOnly)) (Variables|/Game/CustomMaps/UGC1951491250/PMF/Blueprints/Objects/PMF_PavlovIndexs.PMF_PavlovIndexs_C|GetInventoryCharacterBodyMeshOffset _indexs) (Variables|/Game/CustomMaps/UGC1951491250/PMF/Blueprints/Objects/PMF_PavlovIndexs.PMF_PavlovIndexs_C|GetInventoryCharacterHelmetMeshOffset _indexs)))
              (for (_ _array_index) (Rendering|Material|GetMaterials (Utilities|Array|Get(acopy) (Actor|GetComponentsByClass Character "/Script/Engine.SkeletalMeshComponent") _index))
                (Rendering|Material|SetMaterial (Utilities|Array|Get(acopy) (Actor|GetComponentsByClass Character "/Script/Engine.SkeletalMeshComponent") _index) _array_index MaterialToApply))))
          (:Is%20Not%20Valid
            (Logging|AddPMFLogBeta "AddMaterialToCharacter() Material Null" (LocalVariables|Get__WorldContext)))))
      (:Is%20Not%20Valid
        (Logging|AddPMFLogBeta "AddMaterialToCharacter() Character Null" (LocalVariables|Get__WorldContext))))))

(fn HidePavlovGameOverScreen
  (bind ___worldcontext (LocalVariables|Get__WorldContext))
  (bind _localpri (Getters|GetLocalPRI ___worldcontext))
  (bind (_pawn _bisvalid) (Default|GetPlayerPawn _localpri))
  (if _bisvalid
    (for _array_element (Actor|GetAttachedActors _pawn)
      (if (Utilities|Enum|Equal(Enum) (Utilities|GetClassDisplayName (Utilities|GetClass _array_element)) (Variables|/Game/CustomMaps/UGC1951491250/PMF/Blueprints/Objects/PMF_PavlovClassNames.PMF_PavlovClassNames_C|GetPavlovGameOverScreenClassName (Globals|GetPavlovClassNames (LocalVariables|Get__WorldContext))))
        (for _array_element_2 (Actor|GetComponentsByClass _array_element "/Script/UMG.WidgetComponent")
          (for (_ _array_index) (Rendering|Material|GetMaterials _array_element_2)
            (Rendering|Material|SetMaterial _array_element_2 _array_index "/Game/CustomMaps/UGC1951491250/PMF/Materials/M_Nothing.M_Nothing")))))))

(fn GetPavlovClassNames
  (bind _returnvalue (Game|ConstructObjectfromClass "/Game/CustomMaps/UGC1951491250/PMF/Blueprints/Objects/PMF_PavlovClassNames.PMF_PavlovClassNames_C" (LocalVariables|Get__WorldContext)))
  (return _returnvalue))

(fn DestroyPavlovGameOverScreen
  (bind ___worldcontext (LocalVariables|Get__WorldContext))
  (bind _localpri (Getters|GetLocalPRI ___worldcontext))
  (bind (_pawn _bisvalid) (Default|GetPlayerPawn _localpri))
  (if _bisvalid
    (for _array_element (Actor|GetAttachedActors _pawn)
      (if (Utilities|Enum|Equal(Enum) (Utilities|GetClassDisplayName (Utilities|GetClass _array_element)) (Variables|/Game/CustomMaps/UGC1951491250/PMF/Blueprints/Objects/PMF_PavlovClassNames.PMF_PavlovClassNames_C|GetPavlovGameOverScreenClassName (Globals|GetPavlovClassNames (LocalVariables|Get__WorldContext))))
        (Actor|DestroyActor _array_element)))))

(fn GetDirto
  (params (To :type Vector) (From :type Vector) (bNormalize :type Boolean))
  (bind _returnvalue (- To From))
  (if bNormalize
    (return (Math|Vector|Normalize _returnvalue))
    (else
      (return _returnvalue))))

(fn GetDirtoFlat
  (params (To :type Vector) (From :type Vector) (bNormalize :type Boolean))
  (bind ___worldcontext (LocalVariables|Get__WorldContext))
  (return (Maths|GetDirto (Maths|VectorFlat To ___worldcontext) (Maths|VectorFlat From ___worldcontext) bNormalize (LocalVariables|Get__WorldContext))))

(fn VectorFlat
  (params (Vector :type Vector))
  (bind (_x _y) (Math|Vector|BreakVector Vector))
  (return (Math|Vector|MakeVector _x _y 0.0)))