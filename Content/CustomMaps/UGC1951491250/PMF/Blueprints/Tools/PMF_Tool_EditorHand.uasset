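; PMF editor hand tool that fakes a hand's grab interaction, apparently for testing interactables.
; Every Tick it gathers actors overlapping its Sphere that implement PMFI_Interactable and report as interactable.
; It calls Use on the first collected interactable and shows the count and chosen name on two text displays.
; DoInteraction and the construction script are empty.
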(event EventTick
  (params (DeltaSeconds :type Float%20%28single-precision%29))
  (CallFunction|FakeGrabInteraction))

(fn ConstructionScript)

(fn FakeGrabInteraction
  (bind _overlappinginteractables (LocalVariables|GetOverlappingInteractables))
  (bind _returnvalue (Utilities|Array|Length _overlappinginteractables))
  (bind _output (Utilities|Array|Get(acopy) _overlappinginteractables))
  (for _array_element (Collision|GetOverlappingActors (Variables|Default|GetSphere) "/Script/Engine.Actor" :!class /Script/Engine.PrimitiveComponent)
    (if (Utilities|DoesObjectImplementInterface _array_element "/Game/CustomMaps/UGC1951491250/PMF/Blueprints/Interfaces/PMFI_Interactable.PMFI_Interactable_C")
      (bind _bisinteractable (Class|PMFIInteractable|IsInteractable(Message) _array_element))
      (if _bisinteractable
        (Utilities|Array|AddUnique (LocalVariables|GetOverlappingInteractables) _array_element))))
  (if (> _returnvalue 0)
    (Class|PMFIInteractable|UseInteractable(Message) _output)
    (Rendering|Components|TextRender|SetText (Variables|Default|GetInteractablesFound) (Utilities|Text|ToText(String) (Utilities|String|Append "Interactables Found: " (Utilities|String|ToString(Integer) _returnvalue))))
    (Rendering|Components|TextRender|SetText (Variables|Default|GetChosenInteractable) (Utilities|Text|ToText(String) (Utilities|String|Append "Interactable Chosen: " (Utilities|GetDisplayName _output))))
    (return _output)
    (else
      (Rendering|Components|TextRender|SetText (Variables|Default|GetInteractablesFound) (Utilities|Text|MakeLiteralText "Interactables Found: 0"))
      (Rendering|Components|TextRender|SetText (Variables|Default|GetChosenInteractable) (Utilities|Text|MakeLiteralText "No Interactable"))
      (return 0))))

(fn DoInteraction)