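; PMF_PlayerSpawn is a placeable level actor for the PMF custom map that marks a player spawn and tracks its usage.
; It stores an enabled flag, plus the player replication info of the last user and the time of that use.
; Timestamps come from the GameState's server world time, and a getter returns seconds since last use.
; It has no active event logic and only exposes state through functions.
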(event EventBeginPlay)

(event Collision|EventActorBeginOverlap
  (params (OtherActor :type Actor%20Object%20Reference)))

(event EventTick
  (params (DeltaSeconds :type Float%20%28single-precision%29)))

(fn ConstructionScript)

(fn SetSpawnEnabled
  (params (bNewEnabled :type Boolean))
  (Variables|Config|SetbSpawnIsEnabled bNewEnabled))

(fn SpawnUsed
  (params (UserPRI :type PMF%20Player%20Replication%20Info%20Object%20Reference))
  (Variables|Data|SetLastUserPRI UserPRI)
  (Variables|Data|SetLastTimeSpawnWasUsed (GameState|GetServerWorldTimeSeconds (Game|GetGameState))))

(fn GetTimeSinceSpawnWasUsed
  (return (- (GameState|GetServerWorldTimeSeconds (Game|GetGameState)) (Variables|Data|GetLastTimeSpawnWasUsed))))