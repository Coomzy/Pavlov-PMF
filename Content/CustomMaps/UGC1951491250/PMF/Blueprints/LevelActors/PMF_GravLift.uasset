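; PMF_GravLift is a gravity lift level actor that pushes characters upward while they are inside its collision box.
; Entering pawns that are characters get a small upward launch to start them moving.
; Each tick, locally controlled overlapping characters whose vertical velocity is at or below MaxVelZ gain upward velocity from ForceZ scaled by delta time.
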(event EventOnPlayerEnter
  (params (PRI :type PMF%20Player%20Replication%20Info%20Object%20Reference) (Pawn :type Pawn%20Object%20Reference))
  (bind _ascharacter (Utilities|Casting|CastToCharacter Pawn))
  (Character|LaunchCharacter _ascharacter "0, 0,5.000000" false false) ; A little launch might get us going?
)

(event EventTick
  (params (DeltaSeconds :type Float%20%28single-precision%29))
  (for _array_element (Collision|GetOverlappingActors (Variables|Default|GetPlayerCollisionBox) "/Script/Engine.Character" :!class /Script/Engine.PrimitiveComponent)
    (if (<= (.Z (Math|Vector|BreakVector (Transformation|GetVelocity _array_element))) (Variables|Default|GetMaxVelZ))
      (bind _ascharacter (Utilities|Casting|CastToCharacter _array_element))
      (if (Pawn|IsLocallyControlled _ascharacter)
        (CallFunction|AddVelocitytoCharacter _ascharacter (Math|Vector|MakeVector 0.0 0.0 (* DeltaSeconds (Variables|Default|GetForceZ))))))))

(fn ConstructionScript
  (|CallParentFunction))