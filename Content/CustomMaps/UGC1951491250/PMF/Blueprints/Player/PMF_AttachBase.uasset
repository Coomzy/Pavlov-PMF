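; Base Blueprint for player attachments that snap to either the dominant or off-hand controller, chosen by a flag.
; BeginPlay fetches the PMF game logic, runs the empty Initialize hook and binds to the owning PRI's input-refresh event.
; Each refresh re-resolves the controller from PMFPlayerInput and attaches AttachRoot to GetAttachingRoot, which returns that controller here.
; A helper reports whether the chosen hand holds an item.
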(event Custom|RefreshInput
  (CallFunction|AttachRoots))

(event EventBeginPlay
  (|CallParentFunction)
  (CallFunction|GetDataSetup)
  (CallFunction|Initialize)
  (EventDispatchers|BindEventtoRefreshInputs (Variables|Data|GetOwningPRI) (delegate Custom|RefreshInput)))

(fn ConstructionScript)

(fn ControllerHasIteminHand
  (bind _owningpri (Variables|Data|GetOwningPRI))
  (bind _pmfplayerinput (Variables|/Game/CustomMaps/UGC1951491250/PMF/Blueprints/Info/PMF_PlayerReplicationInfo.PMF_PlayerReplicationInfo_C|GetPMFPlayerInput _owningpri))
  (if (Variables|Config|GetbAttachRootToDominantHand)
    (bind _bhasiteminhand (Default|IsDominantHandHoldingItem _pmfplayerinput))
    (return _bhasiteminhand)
    (else
      (bind _bhasiteminhand_2 (Default|IsOffHandHoldingItem _pmfplayerinput))
      (return _bhasiteminhand_2))))

(fn AttachRoots
  (bind _outmotioncontroller (CallFunction|GetAttachingHand))
  (Variables|Default|SetOwningController _outmotioncontroller)
  (bind _attachingroot (CallFunction|GetAttachingRoot))
  (Transformation|AttachComponentToComponent (Variables|Default|GetAttachRoot) _attachingroot "None" "SnapToTarget" "SnapToTarget" "KeepRelative" true))

(fn Initialize)

(fn GetAttachingHand
  (bind _owningpri (Variables|Data|GetOwningPRI))
  (bind _pmfplayerinput (Variables|/Game/CustomMaps/UGC1951491250/PMF/Blueprints/Info/PMF_PlayerReplicationInfo.PMF_PlayerReplicationInfo_C|GetPMFPlayerInput _owningpri))
  (if (Variables|Config|GetbAttachRootToDominantHand)
    (bind _outmotioncontroller (Default|GetDominantController _pmfplayerinput))
    (return _outmotioncontroller)
    (else
      (bind _outmotioncontroller_2 (Default|GetOffController _pmfplayerinput))
      (return _outmotioncontroller_2))))

(fn GetDataSetup
  (CallFunction|SetPMFGameLogicbyRef (Variables|Data|GetPMFGameLogic)))

(fn GetAttachingRoot
  (return (Variables|Default|GetOwningController)))