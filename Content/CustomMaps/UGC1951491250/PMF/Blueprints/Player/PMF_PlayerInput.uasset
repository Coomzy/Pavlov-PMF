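; Per-player VR input handler for PMF in Pavlov, routing scoreboard, trigger and grip presses from both controllers to systems on the owning PRI.
; Triggers drive custom hands, custom items and, on the dominant hand only, the widget interactor; grips drive custom hands, and the off-hand menu button opens the scoreboard.
; Delayed refresh caches controllers and camera from the pawn's components.
; Helpers resolve handedness (default right) and held items via attached actors.
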(event Custom|RefreshInputs
  (Utilities|FlowControl|Delay 0.2)
  (CallFunction|GetControllersandCamera)
  (Default|CallRefreshInputs (Variables|Data|GetOwningPRI)))

(event EventBeginPlay
  (CallFunction|SetPMFGameLogicbyRef (Variables|Data|GetPMFGameLogic))
  (Utilities|FlowControl|Delay 0.3)
  (CallFunction|RefreshInputs))

(event Input|ActionEvents|InputActionScoreboardRight
  (params (Key :type Key%20Structure))
  (:Pressed
    (Inputs-General|InputMenuButton true true))
  (:Released
    (Inputs-General|InputMenuButton true false)))

(event Input|ActionEvents|InputActionScoreboardLeft
  (params (Key :type Key%20Structure))
  (:Pressed
    (Inputs-General|InputMenuButton false true))
  (:Released
    (Inputs-General|InputMenuButton false false)))

(event Input|ActionEvents|InputActionTriggerRight
  (params (Key :type Key%20Structure))
  (:Pressed
    (Inputs-General|InputTriggerButton true true))
  (:Released
    (Inputs-General|InputTriggerButton true false)))

(event Input|ActionEvents|InputActionTriggerLeft
  (params (Key :type Key%20Structure))
  (:Pressed
    (Inputs-General|InputTriggerButton false true))
  (:Released
    (Inputs-General|InputTriggerButton false false)))

(event Input|ActionEvents|InputActionGripToggleLeft
  (params (Key :type Key%20Structure))
  (:Pressed
    (Inputs-General|InputGripButton false true))
  (:Released
    (Inputs-General|InputGripButton false false)))

(event Input|ActionEvents|InputActionGripToggleRight
  (params (Key :type Key%20Structure))
  (:Pressed
    (Inputs-General|InputGripButton true true))
  (:Released
    (Inputs-General|InputGripButton true false)))

(fn ConstructionScript)

(fn GetControllersandCamera
  (for _array_element (Components|GetChildrenComponents (VehicleSound|GetRootComponent (.Pawn (Default|GetPlayerPawn (Variables|Data|GetOwningPRI)))) true)
    (bind _asmotion_controller_component (Utilities|Casting|CastToMotionControllerComponent _array_element)
      (:then
        (switch name (Variables|/Script/HeadMountedDisplay.MotionControllerComponent|GetMotionSource _asmotion_controller_component)
          (:Left
            (Variables|Default|SetControllerL _asmotion_controller_component))
          (:Right
            (Variables|Default|SetControllerR _asmotion_controller_component))))
      (:CastFailed
        (bind _ascamera_component (Utilities|Casting|CastToCameraComponent _array_element))
        (Variables|Default|SetCamera _ascamera_component)))))

(fn GetController
  (params (bGetRightHand :type Boolean))
  (return (select bGetRightHand (Variables|Default|GetControllerR) (Variables|Default|GetControllerL))))

(fn IsRightHanded
  (bind (_playerstatus _bsucceeded) (Default|GetPavlovPlayerStatusbyPRI (Variables|Data|GetPMFGameLogic) (Variables|Data|GetOwningPRI)))
  (if _bsucceeded
    (return (Utilities|Struct|BreakPavlovPlayerStatus _playerstatus))
    (else
      (return true) ; Sorry Lefties, Right Is Default!
    )))

(fn GetDominantController
  (return (select (CallFunction|IsRightHanded) (Variables|Default|GetControllerR) (Variables|Default|GetControllerL))))

(fn GetOffController
  (return (select (CallFunction|IsRightHanded) (Variables|Default|GetControllerL) (Variables|Default|GetControllerR))))

(fn IsControllerHoldingItem
  (params (bCheckRightHand :type Boolean))
  (for _array_element (Actor|GetAttachedActors (Components|GetOwner (select bCheckRightHand (Variables|Default|GetControllerR) (Variables|Default|GetControllerL))))
    (bind _itemid (CallFunction|GetItemIDbyClass (Utilities|GetClass _array_element)))
    (if (Utilities|Enum|NotEqual(Enum) _itemid "NewEnumerator42")
      (return true _itemid)))
  (return false "NewEnumerator42"))

(fn IsDominantHandHoldingItem
  (bind _bhasiteminhand (CallFunction|IsControllerHoldingItem (CallFunction|IsRightHanded)))
  (return _bhasiteminhand))

(fn InputMenuButton
  (params (bIsRightController :type Boolean) (bIsButtonDown :type Boolean))
  (Inputs-Specific|InputScoreboard bIsRightController bIsButtonDown))

(fn InputScoreboard
  (params (bIsRightController :type Boolean) (bIsButtonDown :type Boolean))
  (bind _owningpri (Variables|Data|GetOwningPRI))
  (bind _spawnedscoreboard (Variables|/Game/CustomMaps/UGC1951491250/PMF/Blueprints/Info/PMF_PlayerReplicationInfo.PMF_PlayerReplicationInfo_C|GetSpawnedScoreboard _owningpri))
  (Utilities|ContinueifHandIs (not bIsRightController)
    (:Continue
      (Utilities|IsValid _spawnedscoreboard
        (:Is%20Valid
          (if bIsButtonDown
            (Default|ScoreboardOpen _spawnedscoreboard)
            (else
              (Default|ScoreboardClosed _spawnedscoreboard))))))))

(fn InputTriggerButton
  (params (bIsRightController :type Boolean) (bIsButtonDown :type Boolean))
  (Inputs-Specific|InputCustomHandsTrigger bIsRightController bIsButtonDown)
  (Inputs-Specific|InputWidgetInteractor bIsRightController bIsButtonDown)
  (Inputs-Specific|InputCustomItemTrigger bIsRightController bIsButtonDown))

(fn InputCustomHandsTrigger
  (params (bIsRightController :type Boolean) (bIsButtonDown :type Boolean))
  (bind _owningpri (Variables|Data|GetOwningPRI))
  (bind _pmfcustomhand_l (Variables|/Game/CustomMaps/UGC1951491250/PMF/Blueprints/Info/PMF_PlayerReplicationInfo.PMF_PlayerReplicationInfo_C|GetPMFCustomHand_L _owningpri))
  (bind _pmfcustomhand_r (Variables|/Game/CustomMaps/UGC1951491250/PMF/Blueprints/Info/PMF_PlayerReplicationInfo.PMF_PlayerReplicationInfo_C|GetPMFCustomHand_R _owningpri))
  (bind _returnvalue (select bIsRightController _pmfcustomhand_r _pmfcustomhand_l))
  (Utilities|IsValid _returnvalue
    (:Is%20Valid
      (Default|InputTrigger _returnvalue bIsButtonDown))))

(fn InputWidgetInteractor
  (params (bIsRightController :type Boolean) (bIsButtonDown :type Boolean))
  (bind _owningpri (Variables|Data|GetOwningPRI))
  (bind _spawnedinteractionsystem (Variables|/Game/CustomMaps/UGC1951491250/PMF/Blueprints/Info/PMF_PlayerReplicationInfo.PMF_PlayerReplicationInfo_C|GetSpawnedInteractionSystem _owningpri))
  (Utilities|ContinueifHandIs bIsRightController
    (:Continue
      (Utilities|IsValid _spawnedinteractionsystem
        (:Is%20Valid
          (if bIsButtonDown
            (Default|TriggerPressed _spawnedinteractionsystem)
            (else
              (Default|TriggerReleased _spawnedinteractionsystem))))))))

(fn IsOffHandHoldingItem
  (bind _bhasiteminhand (CallFunction|IsControllerHoldingItem (not (CallFunction|IsRightHanded))))
  (return _bhasiteminhand))

(fn InputCustomHandsGrip
  (params (bIsRightController :type Boolean) (bIsButtonDown :type Boolean))
  (bind _owningpri (Variables|Data|GetOwningPRI))
  (bind _pmfcustomhand_l (Variables|/Game/CustomMaps/UGC1951491250/PMF/Blueprints/Info/PMF_PlayerReplicationInfo.PMF_PlayerReplicationInfo_C|GetPMFCustomHand_L _owningpri))
  (bind _pmfcustomhand_r (Variables|/Game/CustomMaps/UGC1951491250/PMF/Blueprints/Info/PMF_PlayerReplicationInfo.PMF_PlayerReplicationInfo_C|GetPMFCustomHand_R _owningpri))
  (bind _returnvalue (select bIsRightController _pmfcustomhand_r _pmfcustomhand_l))
  (Utilities|IsValid _returnvalue
    (:Is%20Valid
      (Default|InputGrip _returnvalue bIsButtonDown))))

(fn InputGripButton
  (params (bIsRightController :type Boolean) (bIsButtonDown :type Boolean))
  (Inputs-Specific|InputCustomHandsGrip bIsRightController bIsButtonDown))

(fn AreControllersValid
  (return (and (Utilities|IsValid (Variables|Default|GetControllerL)) (Utilities|IsValid (Variables|Default|GetControllerR)))))

(fn IsControllerHoldingActor
  (params (CheckingActor :type Actor%20Object%20Reference) (bCheckRightHand :type Boolean))
  (Utilities|IsValid CheckingActor
    (:Is%20Valid
      (return (== (Actor|GetAttachParentActor CheckingActor) (Components|GetOwner (select bCheckRightHand (Variables|Default|GetControllerR) (Variables|Default|GetControllerL))))))
    (:Is%20Not%20Valid
      (return false))))

(fn GetControllerDominant
  (params (bGetDominant :type Boolean))
  (bind _bisrighthanded (CallFunction|IsRightHanded))
  (bind _outmotioncontroller (CallFunction|GetController (select bGetDominant _bisrighthanded (not _bisrighthanded))))
  (return _outmotioncontroller))

(fn InputCustomItemTrigger
  (params (bIsRightController :type Boolean) (bIsButtonDown :type Boolean))
  (bind _owningpri (Variables|Data|GetOwningPRI))
  (bind (_bfoundcustomitem _customitem) (Default|GetCustomItemonPlayer _owningpri bIsRightController))
  (if _bfoundcustomitem
    (if bIsButtonDown
      (Default|StartUseItem _customitem)
      (else
        (Default|FinishUseItem _customitem)))))