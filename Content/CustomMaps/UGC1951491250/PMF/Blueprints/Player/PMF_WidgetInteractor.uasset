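; PMF player widget interactor that gives a laser pointer for clicking UI widgets, by default while an interactable or admin-panel scoreboard is open.
; Each tick it checks scoreboard state, an empty controller hand and an optional player-role requirement, toggling pointer visibility and hit testing.
; The line mesh stretches to the hit or maximum distance, with a torus reticle aligned to the hit normal.
; Trigger presses become left clicks; release always fires.
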(event Custom|TriggerPressed
  (bind _bison (CallFunction|IsInteractionSystemon))
  (if _bison
    (Class|WidgetInteractionComponent|PressPointerKey (Variables|Default|GetWidgetInteraction) "LeftMouseButton")))

(event Custom|TriggerReleased
  (Class|WidgetInteractionComponent|ReleasePointerKey (Variables|Default|GetWidgetInteraction) "LeftMouseButton") ; I think it should always release the key press
)

(event EventTick
  (params (DeltaSeconds :type Float%20%28single-precision%29))
  (|CallParentFunction DeltaSeconds)
  (CallFunction|UpdateInteractionSystem))

(event EventInitialize
  (CallFunction|SetupWidgetInteraction))

(fn ConstructionScript)

(fn UpdateInteractionSystem
  (bind _widgetinteraction (Variables|Default|GetWidgetInteraction))
  (bind _widgettorusmesh (Variables|Default|GetWidgetTorusMesh))
  (bind _widgetlinemeshstartingscale (Variables|Data|GetWidgetLineMeshStartingScale))
  (bind _widgetlinemeshstartingscale_2 (Variables|Data|GetWidgetLineMeshStartingScale))
  (bind _widgetinteraction_2 (Variables|Default|GetWidgetInteraction))
  (bind (_x _y _z) (Math|Vector|BreakVector _widgetlinemeshstartingscale_2))
  (bind _returnvalue (Class|WidgetInteractionComponent|GetLastHitResult _widgetinteraction))
  (bind (_x_2 _y_2 _z_2) (Math|Vector|BreakVector _widgetlinemeshstartingscale))
  (bind (_bblockinghit _binitialoverlap _time _distance _location _impactpoint _normal _impactnormal) (Collision|BreakHitResult _returnvalue))
  (bind _bison (CallFunction|IsInteractionSystemon))
  (if _bison
    (Utilities|FlowControl|Sequence
      (:then_0
        (Variables|/Script/UMG.WidgetInteractionComponent|SetbEnableHitTesting _widgetinteraction_2 true)
        (Development|SetHiddeninGame _widgetinteraction_2 false true))
      (:then_1
        (CallFunction|UpdateInteractionDistance))
      (:then_2
        (if (not _bblockinghit) ; Did We Hit Nothing?
          (Transformation|SetRelativeScale3D (Variables|Default|GetWidgetLineMesh) (Math|Vector|MakeVector (/ (Variables|Data|GetInteractionSystemDistance) 2e+02) _y _z))
          (Transformation|SetRelativeLocationAndRotation (Variables|Default|GetWidgetTorusMesh) (Math|Vector|MakeVector (Variables|Data|GetInteractionSystemDistance) 0.0 0.0) "0, 0, 0" false false)
          (else
            (Transformation|SetRelativeScale3D (Variables|Default|GetWidgetLineMesh) (Math|Vector|MakeVector (/ _distance 2e+02) _y_2 _z_2))
            (Transformation|SetRelativeLocation _widgettorusmesh (Math|Vector|MakeVector _distance 0.0 0.0) false false)
            (Transformation|SetWorldRotation _widgettorusmesh (Math|Conversions|RotationFromXVector _impactnormal) false false)))))
    (else
      (Development|SetHiddeninGame (Variables|Default|GetWidgetInteraction) true true)
      (Variables|/Script/UMG.WidgetInteractionComponent|SetbEnableHitTesting (Variables|Default|GetWidgetInteraction) false))))

(fn SetupWidgetInteraction
  (Variables|/Script/UMG.WidgetInteractionComponent|SetInteractionDistance (Variables|Default|GetWidgetInteraction) (Variables|Data|GetInteractionSystemDistance))
  (Variables|Data|SetWidgetLineMeshStartingScale (Variables|/Script/Engine.SceneComponent|GetRelativeScale3D (Variables|Default|GetWidgetLineMesh))))

(fn IsInteractionSystemon
  (bind _owningpri (Variables|Default|GetOwningPRI))
  (bind _owningpri_2 (Variables|Default|GetOwningPRI))
  (bind _customscoreboardclass (Variables|/Game/CustomMaps/UGC1951491250/PMF/Blueprints/Info/PMF_PlayerReplicationInfo.PMF_PlayerReplicationInfo_C|GetCustomScoreboardClass _owningpri_2))
  (bind _spawnedscoreboard (Variables|/Game/CustomMaps/UGC1951491250/PMF/Blueprints/Info/PMF_PlayerReplicationInfo.PMF_PlayerReplicationInfo_C|GetSpawnedScoreboard _owningpri))
  (bind (_bdestroydebugwidget _bscoreboardisopen _buseadminpanel _bisinteractable) (Utilities|GetClassDefaults _customscoreboardclass))
  (if (Variables|Config|GetbMustHaveRole)
    (if (CallFunction|IsRequiredRole)
      _
      (else
        (return false))))
  (if (or _buseadminpanel _bisinteractable) ; Default Behaviour Is When Scoreboard Is Open
    (Utilities|IsValid _spawnedscoreboard
      (:Is%20Valid
        (if (Variables|/Game/CustomMaps/UGC1951491250/PMF/Blueprints/Player/PMF_CustomScoreboard.PMF_CustomScoreboard_C|GetbScoreboardIsOpen _spawnedscoreboard)
          (bind _bhasiteminhand (CallFunction|ControllerHasIteminHand))
          (return (not _bhasiteminhand))
          (else
            _)))
      (:Is%20Not%20Valid
        _))
    (return false)
    (else
      (return false))))

(fn UpdateInteractionDistance
  (bind _output_get (Variables|Data|SetInteractionSystemDistance (CallFunction|GetInteractionDistance)))
  (Variables|/Script/UMG.WidgetInteractionComponent|SetInteractionDistance (Variables|Default|GetWidgetInteraction) _output_get))

(fn GetInteractionDistance
  (return (Variables|Config|GetInteractionSystemDistanceDefault)))

(fn IsRequiredRole
  (if (Variables|Config|GetbMustHaveRole)
    (return (<= (Default|GetPlayerRole (CallFunction|GetLocalPRI)) (Variables|Config|GetRoleRequired)))
    (else
      (return true))))