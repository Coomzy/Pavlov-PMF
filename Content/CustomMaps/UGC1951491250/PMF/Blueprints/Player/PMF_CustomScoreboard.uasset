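; PMF custom player scoreboard that shows or hides its root on open and close, with optional debug and admin widgets.
; Setup starts it closed and destroys the debug widget if flagged or in live builds without a keep override, and the admin widget if disabled.
; On input refresh, the debug widget is shown only to roled players and the admin widget only to admins.
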(event Custom|ScoreboardClosed
  (Development|SetHiddeninGame (Variables|Default|GetScoreboardRoot) true true)
  (Variables|Data|SetbScoreboardIsOpen false))

(event Custom|ScoreboardOpen
  (Development|SetHiddeninGame (Variables|Default|GetScoreboardRoot) false true)
  (Variables|Data|SetbScoreboardIsOpen true))

(event EventInitialize
  (CallFunction|SetupScoreboard))

(event EventRefreshInput
  (|CallParentFunction)
  (CallFunction|RefreshScoreboard))

(fn ConstructionScript)

(fn SetupScoreboard
  (CallFunction|ScoreboardClosed)
  (Utilities|FlowControl|Sequence
    (:then_0
      (if (Variables|Config|GetbDestroyDebugWidget) ; Debug Menu?
        (Components|DestroyComponent (Variables|Default|GetWidgetDebug))
        (else
          (Utilities|IsLiveBuild
            (:Is%20Live%20Build
              (if (not (Variables|Config|GetbKeepDebugWidgetInLiveBuild))
                (Components|DestroyComponent (Variables|Default|GetWidgetDebug))))))))
    (:then_1
      (if (not (Variables|Config|GetbUseAdminPanel)) ; Enable/Disable Admin Panel
        (Components|DestroyComponent (Variables|Default|GetWidgetAdmin))))))

(fn RefreshScoreboard
  (Utilities|FlowControl|Sequence
    (:then_0
      (Utilities|IsValid (Variables|Default|GetWidgetDebug)
        (:Is%20Valid
          (Utilities|IsLiveBuild
            (:Not%20Live%20Build
              (Rendering|SetVisibility (Variables|Default|GetWidgetDebug) (Default|IsRoledPlayer (Variables|Default|GetOwningPRI)) false :!label _label))
            (:Is%20Live%20Build
              (if (Variables|Config|GetbKeepDebugWidgetInLiveBuild)
                (goto _label)))))))
    (:then_1
      (Utilities|IsValid (Variables|Default|GetWidgetAdmin)
        (:Is%20Valid
          (Rendering|SetVisibility (Variables|Default|GetWidgetAdmin) (Default|IsAdmin (Variables|Default|GetOwningPRI)) false))))))