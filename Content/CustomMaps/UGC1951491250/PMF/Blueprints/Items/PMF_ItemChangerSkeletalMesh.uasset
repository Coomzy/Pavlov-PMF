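; Actor that replaces the look of its owning item's skeletal mesh with a custom skeletal mesh, destroying itself if no owner or mesh is found.
; On BeginPlay it blanks the original's materials with an invisible-style M_Nothing instance and snaps the custom mesh onto it, offset sideways in debug mode.
; Drop and pickup events swap the original's mesh asset, an admittedly broken highlight fix.
; Helper functions expose the original mesh's bone transforms in component space.
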(event EventBeginPlay
  (bind _returnvalue (Components|GetOwner))
  (Utilities|IsValid _returnvalue
    (:Is%20Valid
      (bind _output_get (Variables|Default|SetOriginalItemSK_Comp (Actor|GetComponentbyClass _returnvalue "/Script/Engine.SkeletalMeshComponent")))
      (Utilities|IsValid _output_get
        (:Is%20Valid
          (Variables|Data|SetOriginalItem_SK (Variables|/Script/Engine.SkinnedMeshComponent|GetSkeletalMesh (Variables|Default|GetOriginalItemSK_Comp)))
          (for (_ _array_index) (Rendering|Material|GetMaterials (Variables|Default|GetOriginalItemSK_Comp))
            (if (not (Variables|Default|GetbDebugVisuals))
              (bind _returnvalue_2 (Rendering|Material|CreateDynamicMaterialInstance "/Game/CustomMaps/UGC1951491250/PMF/Materials/M_Nothing.M_Nothing" "Nothing" :!class /Script/Engine.KismetMaterialLibrary))
              (Rendering|Material|SetMaterial (Variables|Default|GetOriginalItemSK_Comp) _array_index _returnvalue_2)))
          (Transformation|AttachComponentToComponent (Variables|Default|GetCustomItemSK_Comp) (Variables|Default|GetOriginalItemSK_Comp) "None" "SnapToTarget" "SnapToTarget" "SnapToTarget" true)
          (if (Variables|Default|GetbDebugVisuals)
            (Transformation|SetRelativeLocation (Variables|Default|GetCustomItemSK_Comp) "0,15.000000, 0" false false)))
        (:Is%20Not%20Valid
          (CallFunction|AddPMFLog (Utilities|String|Append "No Skeletal Mesh Found On " (Utilities|GetDisplayName (Components|GetOwner)) " for " (Utilities|GetDisplayName self)))
          (Actor|DestroyActor))))
    (:Is%20Not%20Valid
      (CallFunction|AddPMFLog (Utilities|String|Append "No Owner Found On " (Utilities|GetDisplayName self)))
      (Actor|DestroyActor))))

(event EventAttemptedDrop
  (Class|SkinnedMeshComponent|SetSkeletalMesh (Variables|Default|GetOriginalItemSK_Comp) (Variables|/Script/Engine.SkinnedMeshComponent|GetSkeletalMesh (Variables|Default|GetCustomItemSK_Comp)) true) ; This is an attempt to try and fix the wrong highlight mesh bug but it's fucked, if you fix it let me know
  (CallFunction|AddPMFLog "AttemptedDrop()"))

(event EventAttemptedPickup
  (Class|SkinnedMeshComponent|SetSkeletalMesh (Variables|Default|GetOriginalItemSK_Comp) (Variables|Data|GetOriginalItem_SK) true)
  (CallFunction|AddPMFLog "AttemptedPickup()"))

(fn ConstructionScript)

(fn GetBoneLocationbyName
  (params (BoneName :type Name) (Loc :type Vector%20%28by%20ref%29))
  (bind _originalitemsk_comp (Variables|Default|GetOriginalItemSK_Comp))
  (bind _returnvalue (Transformation|GetSocketTransform _originalitemsk_comp BoneName "RTS_Component"))
  (bind _location (Math|Transform|BreakTransform _returnvalue))
  (|SetBy-RefVar Loc _location)
  (return _location))

(fn GetBoneRotationbyName
  (params (BoneName :type Name) (Rot :type Rotator%20%28by%20ref%29))
  (bind _originalitemsk_comp (Variables|Default|GetOriginalItemSK_Comp))
  (bind _returnvalue (Transformation|GetSocketTransform _originalitemsk_comp BoneName "RTS_Component"))
  (bind _rotation (Math|Transform|BreakTransform _returnvalue))
  (|SetBy-RefVar Rot _rotation)
  (return _rotation))

(fn GetBoneLocationandRotationbyName
  (params (BoneName :type Name) (Loc :type Vector%20%28by%20ref%29) (Rot :type Rotator%20%28by%20ref%29))
  (bind _originalitemsk_comp (Variables|Default|GetOriginalItemSK_Comp))
  (bind _returnvalue (Transformation|GetSocketTransform _originalitemsk_comp BoneName "RTS_Component"))
  (bind (_location _rotation) (Math|Transform|BreakTransform _returnvalue))
  (|SetBy-RefVar Loc _location)
  (|SetBy-RefVar Rot _rotation)
  (return _location _rotation))