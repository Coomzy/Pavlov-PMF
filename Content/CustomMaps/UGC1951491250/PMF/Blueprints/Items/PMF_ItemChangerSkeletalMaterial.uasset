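; PMF item helper actor that overrides every material on its owner's skeletal mesh with a single configured material.
; On BeginPlay it finds the owner's SkeletalMeshComponent and sets each material slot to MaterialToSet, logging and destroying itself if the owner or mesh is missing.
; It also provides functions that return a named bone's component-space location, rotation or both from that mesh, writing results to by-ref variables as well.
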(event EventBeginPlay
  (bind _returnvalue (Components|GetOwner))
  (Utilities|IsValid _returnvalue
    (:Is%20Valid
      (bind _output_get (Variables|Default|SetOriginalItemSK_Comp (Actor|GetComponentbyClass _returnvalue "/Script/Engine.SkeletalMeshComponent")))
      (Utilities|IsValid _output_get
        (:Is%20Valid
          (for (_ _array_index) (Rendering|Material|GetMaterials (Variables|Default|GetOriginalItemSK_Comp))
            (Rendering|Material|SetMaterial (Variables|Default|GetOriginalItemSK_Comp) _array_index (Variables|Default|GetMaterialToSet))))
        (:Is%20Not%20Valid
          (CallFunction|AddPMFLog (Utilities|String|Append "No Skeletal Mesh Found On " (Utilities|GetDisplayName (Components|GetOwner)) " for " (Utilities|GetDisplayName self)))
          (Actor|DestroyActor))))
    (:Is%20Not%20Valid
      (CallFunction|AddPMFLog (Utilities|String|Append "No Owner Found On " (Utilities|GetDisplayName self)))
      (Actor|DestroyActor))))

(fn ConstructionScript)

(fn GetBoneLocationbyName
  (params (BoneName :type Name) (Loc :type Vector%20%28by%20ref%29))
  (bind _originalitemsk_comp (Variables|Default|GetOriginalItemSK_Comp))
  (bind _returnvalue (Transformation|GetSocketTransform _originalitemsk_comp BoneName "RTS_Component"))
  (bind _location (Math|Transform|BreakTransform _returnvalue))
  (|SetBy-RefVar Loc _location)
  (return _location))

(fn GetBoneRotationbyName
  (params (BoneName :type Name) (Rot :type Rotator%20%28by%20ref%29))
  (bind _originalitemsk_comp (Variables|Default|GetOriginalItemSK_Comp))
  (bind _returnvalue (Transformation|GetSocketTransform _originalitemsk_comp BoneName "RTS_Component"))
  (bind _rotation (Math|Transform|BreakTransform _returnvalue))
  (|SetBy-RefVar Rot _rotation)
  (return _rotation))

(fn GetBoneLocationandRotationbyName
  (params (BoneName :type Name) (Loc :type Vector%20%28by%20ref%29) (Rot :type Rotator%20%28by%20ref%29))
  (bind _originalitemsk_comp (Variables|Default|GetOriginalItemSK_Comp))
  (bind _returnvalue (Transformation|GetSocketTransform _originalitemsk_comp BoneName "RTS_Component"))
  (bind (_location _rotation) (Math|Transform|BreakTransform _returnvalue))
  (|SetBy-RefVar Loc _location)
  (|SetBy-RefVar Rot _rotation)
  (return _location _rotation))