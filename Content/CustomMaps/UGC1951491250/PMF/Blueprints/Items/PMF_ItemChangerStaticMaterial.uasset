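; PMF item actor that overrides the static mesh materials of the actor that owns it.
; On BeginPlay it finds the owner's StaticMeshComponent and sets every material slot to MaterialToSet.
; If the owner or mesh is missing, it writes a PMF log message and destroys itself.
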(event EventBeginPlay
  (bind _returnvalue (Components|GetOwner))
  (Utilities|IsValid _returnvalue
    (:Is%20Valid
      (bind _output_get (Variables|Default|SetOriginalItemSM_Comp (Actor|GetComponentbyClass _returnvalue "/Script/Engine.StaticMeshComponent")))
      (Utilities|IsValid _output_get
        (:Is%20Valid
          (for (_ _array_index) (Rendering|Material|GetMaterials (Variables|Default|GetOriginalItemSM_Comp))
            (Rendering|Material|SetMaterial (Variables|Default|GetOriginalItemSM_Comp) _array_index (Variables|Default|GetMaterialToSet))))
        (:Is%20Not%20Valid
          (CallFunction|AddPMFLog (Utilities|String|Append "No Static Mesh Found On " (Utilities|GetDisplayName (Components|GetOwner)) " for " (Utilities|GetDisplayName self)))
          (Actor|DestroyActor))))
    (:Is%20Not%20Valid
      (CallFunction|AddPMFLog (Utilities|String|Append "No Owner Found On " (Utilities|GetDisplayName self)))
      (Actor|DestroyActor))))

(fn ConstructionScript)