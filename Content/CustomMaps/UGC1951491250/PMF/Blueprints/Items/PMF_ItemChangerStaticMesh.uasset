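; PMF item changer actor that replaces the visible static mesh of its owning item with its own custom mesh component.
; On BeginPlay it blanks each material on the owner's StaticMeshComponent with M_Nothing, then snaps the custom mesh onto that component.
; DebugVisuals keeps the original materials and offsets the custom mesh sideways.
; Without a valid owner or mesh component, it logs to the PMF log and destroys itself.
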(event EventBeginPlay
  (bind _returnvalue (Components|GetOwner))
  (Utilities|IsValid _returnvalue
    (:Is%20Valid
      (bind _output_get (Variables|Default|SetOriginalItemSM_Comp (Actor|GetComponentbyClass _returnvalue "/Script/Engine.StaticMeshComponent")))
      (Utilities|IsValid _output_get
        (:Is%20Valid
          (for (_ _array_index) (Rendering|Material|GetMaterials (Variables|Default|GetOriginalItemSM_Comp))
            (if (not (Variables|Default|GetbDebugVisuals))
              (Rendering|Material|SetMaterial (Variables|Default|GetOriginalItemSM_Comp) _array_index "/Game/CustomMaps/UGC1951491250/PMF/Materials/M_Nothing.M_Nothing")))
          (Transformation|AttachComponentToComponent (Variables|Default|GetCustomItemSM_Comp) (Variables|Default|GetOriginalItemSM_Comp) "None" "SnapToTarget" "SnapToTarget" "SnapToTarget" true)
          (if (Variables|Default|GetbDebugVisuals)
            (Transformation|SetRelativeLocation (Variables|Default|GetCustomItemSM_Comp) "0,15.000000, 0" false false)))
        (:Is%20Not%20Valid
          (CallFunction|AddPMFLog (Utilities|String|Append "No Static Mesh Found On " (Utilities|GetDisplayName (Components|GetOwner)) " for " (Utilities|GetDisplayName self)))
          (Actor|DestroyActor))))
    (:Is%20Not%20Valid
      (CallFunction|AddPMFLog (Utilities|String|Append "No Owner Found On " (Utilities|GetDisplayName self)))
      (Actor|DestroyActor))))

(fn ConstructionScript)