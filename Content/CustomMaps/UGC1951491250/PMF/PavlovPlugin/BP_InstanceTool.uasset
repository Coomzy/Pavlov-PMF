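; BP_InstanceTool is a utility actor that converts placed StaticMeshActors using a chosen mesh into instances on one Hierarchical Instanced Static Mesh component.
; GenerateInstances scans all StaticMeshActors, adds a world-space instance for each match to MeshToFind, and can destroy the originals.
; Existing instances are cleared first unless AddToHISM is set.
; A separate, caution-flagged event clears all instances.
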(event Custom|Generate%20Instances
  (bind _hierarchicalinstancedstaticmesh (Variables|Default|GetHierarchicalInstancedStaticMesh))
  (bind _outactors (Actor|GetAllActorsOfClass "/Script/Engine.StaticMeshActor"))
  (bind _output_get (Variables|Default|SetStaticMeshActors _outactors))
  (if (>= (Utilities|Array|Length _output_get) 1)
    (if (Variables|Default|GetAddToHISM)
      _
      (else
        (Components|InstancedStaticMesh|ClearInstances _hierarchicalinstancedstaticmesh)))
    (Components|StaticMesh|SetStaticMesh _hierarchicalinstancedstaticmesh (Variables|Default|GetMeshToFind))
    (bind _arrayelement (Utilities|Array|ReverseforEachLoop (Variables|Default|GetStaticMeshActors))
      (:LoopBody
        (if (== (Variables|/Script/Engine.StaticMeshComponent|GetStaticMesh (Variables|/Script/Engine.StaticMeshActor|GetStaticMeshComponent _arrayelement)) (Variables|Default|GetMeshToFind))
          (Class|InstancedStaticMeshComponent|AddInstanceWorldSpace (Variables|Default|GetHierarchicalInstancedStaticMesh) (Transformation|GetActorTransform _arrayelement))
          (if (Variables|Default|GetDestroyFoundActors)
            (Actor|DestroyActor _arrayelement)))))))

(event Custom|Clear%20HISM:%20USE%20WITH%20CAUTION
  (Components|InstancedStaticMesh|ClearInstances (Variables|Default|GetHierarchicalInstancedStaticMesh)))

(fn ConstructionScript)