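; An interactable swinging door for a Pavlov custom map that any user can toggle open or closed.
; Use flips the IsDoorOpen state, and round start can optionally reset it to a configured default.
; The state's RepNotify calls UpdateDoorState, which snaps the Door's relative yaw to the open or closed angle with no animation.
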(event EventUseInteractable
  (params (UserPRI :type PMF%20Player%20Replication%20Info%20Object%20Reference) (UserCPI :type PMF%20Character%20Proxy%20Info%20Object%20Reference) (UserCustomHand :type PMF%20Custom%20Hand%20Object%20Reference))
  (Variables|DataReplicated|SetbIsDoorOpen (not (Variables|DataReplicated|GetbIsDoorOpen))))

(event EventRoundStarting
  (if (Variables|Config|GetbUpdateDoorStateOnRoundStart)
    (Variables|DataReplicated|SetbIsDoorOpen (Variables|Config|GetbDoorIsOpenOnRoundStart))))

(fn ConstructionScript
  (bind _arrow (Variables|Default|GetArrow))
  (if true
    (Rendering|SetVisibility _arrow true false)
    (else
      (Rendering|SetVisibility _arrow false false))))

(fn UpdateDoorState
  (Transformation|SetRelativeRotation (Variables|Default|GetDoor) (Math|Rotator|MakeRotator 0.0 0.0 (Math|Float|SelectFloat (Variables|Config|GetDoorOpenAngle) (Variables|Config|GetDoorClosedAngle) (Variables|DataReplicated|GetbIsDoorOpen))) false false))

(fn OnRepBIsDoorOpen
  (CallFunction|UpdateDoorState))

(fn IsInteractable
  (params (UserPRI :type PMF%20Player%20Replication%20Info%20Object%20Reference) (UserCPI :type PMF%20Character%20Proxy%20Info%20Object%20Reference) (UserCustomHand :type PMF%20Custom%20Hand%20Object%20Reference))
  (return true))